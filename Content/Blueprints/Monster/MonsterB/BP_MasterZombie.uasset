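; Master zombie Blueprint that handles camera-aligned rotation, a death dissolve and surface displacement data.
; Every tick it sets its Rotation component's world rotation to the player camera's rotation.
; DeadEvent plays a timeline that drives the mesh materials' dissolve parameter, then destroys the actor.
; AddDisplacementShapeData feeds shapes from the mesh to the Infinity displacement component, while GetDisplacementTexture is left empty.
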(event `self.ReceiveTick`
  (params (DeltaSeconds :type "Float (single-precision)"))
  (`self.CameraTick` DeltaSeconds))

(event `DeadEvent`
  (bind (_direction _disslove) (`Timeline|타임라인_0` :!via `PlayFromStart`)
    (:`Update`
      (`MeshComponent.SetScalarParameterValueOnMaterials` (`self.Mesh`) "디졸브" _disslove))
    (:`Finished`
      (`self.K2_DestroyActor`))))

(event `CameraTick`
  (params (DeltaSeconds :type "Float (double-precision)"))
  ;[1 1 1] 카메라 각도를 읽어와서 그대로 설정하기.
  (`SceneComponent.K2_SetWorldRotation` (`self.Rotation`) (`PlayerCameraManager.GetCameraRotation` (`GameplayStatics.GetPlayerCameraManager` 0)) false false))

(fn `AddDisplacementShapeData`
  (params (Stack :type "Array of /Game/Assets/InfinityWeather/Displacement/Blueprints/BS_DisplacementShape Structure (by ref)"))
  (returns (Added :type Boolean))
  (`/Game/Assets/InfinityWeather/Displacement/Blueprints/BP_InfinityDisplacementComponent.AddDisplacementShapeData` (`self.BP_InfinityDisplacementComponent`) Stack (`self.Mesh`))
  (return true))

(fn `GetDisplacementTexture`
  (returns (Texture :type "Texture2D Object Reference"))
  (return null))

(fn `UserConstructionScript`)