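; BP_Granade is a grenade actor that explodes on a fixed fuse shortly after spawning.
; BeginPlay starts a one-shot timer, and Detonate spawns the explosion actor and an attenuated sound at its location.
; Only the authority then applies full radial damage with a prevention trace channel and destroys the grenade.
; The damage instigator is always player controller 0 rather than the thrower.
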(event `self.ReceiveBeginPlay`
  (`KismetSystemLibrary.K2_SetTimerDelegate` (delegate `Detonate`) 2.0))

(event `Detonate`
  (`|SpawnActorFromClass` "/Game/Blueprints/Character/Explosion.Explosion_C" (`self.GetTransform`) "Undefined" "OverrideRootScale" null null)
  (`GameplayStatics.SpawnSoundAtLocation` "/Game/Blueprints/Character/Explosion_Sound_Cue.Explosion_Sound_Cue" (`self.K2_GetActorLocation`) (struct) 1.0 1.0 0.0 "/Game/Blueprints/Character/Explosion_Attenuation.Explosion_Attenuation" null)
  (`/Engine/EditorBlueprintResources/ActorMacros.Switch Has Authority`
    (:`Authority`
      (`GameplayStatics.ApplyRadialDamage` :`BaseDamage` 25.0 :`Origin` (`self.K2_GetActorLocation`) :`DamageRadius` 500.0 :`DamageTypeClass` "/Script/TeamPortfolio.BulletDamageType" :`DamageCauser` self :`InstigatedByController` (`GameplayStatics.GetPlayerController` 0) :`bDoFullDamage` true :`DamagePreventionChannel` "ECC_GameTraceChannel3")
      (`self.K2_DestroyActor`))))

(fn `UserConstructionScript`)