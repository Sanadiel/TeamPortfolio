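; BP_MasterLobby_GM is the lobby game mode that repositions players by team and can enable a UI test mode.
; The replace event loops over all BP_PlayerController_BossTest controllers and teleports each controlled pawn to the "Defence" or "Offence" player start, chosen by whether the controller carries the Defence tag.
; SettingTest turns on UITestMode on the first player's controller and runs its UI test setup.
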(event `self.ReceiveBeginPlay`)

(event `replace`
  ;[1 1 1] replace
  (bind _outactors (`GameplayStatics.GetAllActorsOfClass` "/Game/Blueprints/Boss/BP_PlayerController_BossTest.BP_PlayerController_BossTest_C"))
  (for _array_element _outactors
    ;;[1 1 1] 수비자입니까
    (if (`self.ActorHasTag` _array_element "Defence")
      ;;[1 1 1] 수비자
      (`self.K2_SetActorTransform` (`Controller.K2_GetPawn` _array_element) (`self.GetTransform` (`self.K2_FindPlayerStart` _array_element "Defence")) false false)
      (else
        ;;[1 1 1] 공격자
        (`self.K2_SetActorTransform` (`Controller.K2_GetPawn` _array_element) (`self.GetTransform` (`self.K2_FindPlayerStart` _array_element "Offence")) false false)))))

(event `SettingTest`
  (bind _asbp_player_controller_boss_test (cast `/Game/Blueprints/Boss/BP_PlayerController_BossTest` (`GameplayStatics.GetPlayerController` 0)))
  (set `UI_PC.UITestMode` true _asbp_player_controller_boss_test)
  (`UI_PC.SettingUI_TEST` _asbp_player_controller_boss_test))

(fn `UserConstructionScript`)