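; SelectButton is a lobby pressure-button actor that sinks when the player pawn begins overlapping it and rises when the overlap ends.
; The overlap events call DownAction and UpAction, which move the Main component along relative Z using FInterpTo.
; Each action re-calls itself after a short Delay instead of using Tick or a Timeline, then snaps to its end height.
; It only animates and prints debug strings, with no selection logic.
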(event `DownAction`
  (`KismetSystemLibrary.PrintString` "down")
  (`SceneComponent.K2_SetRelativeLocation` (`self.Main`) (`KismetMathLibrary.MakeVector` 0.0 0.0 (`KismetMathLibrary.FInterpTo` (.z (.location (`SceneComponent.GetRelativeTransform` (`self.Main`)))) (`self.DownMax`) (`GameplayStatics.GetWorldDeltaSeconds`) 50.0)) false false)
  (if (> (.z (.location (`SceneComponent.GetRelativeTransform` (`self.Main`)))) -15.0)
    (`KismetSystemLibrary.Delay` 0.05)
    (`self.DownAction`)
    (else
      (`SceneComponent.K2_SetRelativeLocation` (`self.Main`) (0.0 0.0 -15.0) false false)
      (`KismetSystemLibrary.PrintString` "Down End"))))

(event `UpAction`
  (`KismetSystemLibrary.PrintString` "up")
  (`SceneComponent.K2_SetRelativeLocation` (`self.Main`) (`KismetMathLibrary.MakeVector` 0.0 0.0 (`KismetMathLibrary.FInterpTo` (.z (.location (`SceneComponent.GetRelativeTransform` (`self.Main`)))) 0.0 (`GameplayStatics.GetWorldDeltaSeconds`) 50.0)) false false)
  (if (< (.z (.location (`SceneComponent.GetRelativeTransform` (`self.Main`)))) 0.0)
    (`KismetSystemLibrary.Delay` 0.05)
    (`self.UpAction`)
    (else
      (`SceneComponent.K2_SetRelativeLocation` (`self.Main`) (0.0 0.0 0.0) false false)
      (`KismetSystemLibrary.PrintString` "Up End"))))

(event `self.Box.OnComponentBeginOverlap`
  (params (OverlappedComponent :type "PrimitiveComponent Object Reference") (OtherActor :type "Actor Object Reference") (OtherComp :type "PrimitiveComponent Object Reference") (OtherBodyIndex :type Integer) (bFromSweep :type Boolean) (SweepResult :type "HitResult Structure (by ref)")))

(event `self.ReceiveActorBeginOverlap`
  (params (OtherActor :type "Actor Object Reference"))
  (if (== OtherActor (`GameplayStatics.GetPlayerPawn` 0))
    (`self.DownAction`)))

(event `self.Box.OnComponentEndOverlap`
  (params (OverlappedComponent :type "PrimitiveComponent Object Reference") (OtherActor :type "Actor Object Reference") (OtherComp :type "PrimitiveComponent Object Reference") (OtherBodyIndex :type Integer)))

(event `self.ReceiveActorEndOverlap`
  (params (OtherActor :type "Actor Object Reference"))
  (if (== OtherActor (`GameplayStatics.GetPlayerPawn` 0))
    (`self.UpAction`)))

(fn `UserConstructionScript`)