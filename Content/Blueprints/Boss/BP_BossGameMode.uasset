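; Game mode for the boss mode that tracks objective actors and declares the normal players' win when none remain.
; On BeginPlay it gathers all BP_ObjectiveActor instances and binds to their destroyed event.
; Each destruction re-queries the remaining objectives, then tells every BP_PlayerController_BossTest to show game-over UI if none are left, or otherwise call SaySomething.
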(event `self.ReceiveBeginPlay`
  (bind _outactors (`GameplayStatics.GetAllActorsOfClass` "/Game/Blueprints/Boss/BPforTest/BP_ObjectiveActor.BP_ObjectiveActor_C"))
  (set `self.ObjectiveActorArray` _outactors)
  (add `self.WhenObjectiveDestroyed` (delegate `OnObjectiveDestroyed`)))

(event `OnObjectiveDestroyed`
  (bind _outactors (`GameplayStatics.GetAllActorsOfClass` "/Game/Blueprints/Boss/BPforTest/BP_ObjectiveActor.BP_ObjectiveActor_C"))
  (bind _output_get (set `self.ObjectiveActorArray` _outactors))
  (if (<= (`KismetArrayLibrary.Array_Length` _output_get) 0)
    (`KismetSystemLibrary.PrintString` "Normal Players Win!")
    (bind _outactors_2 (`GameplayStatics.GetAllActorsOfClass` "/Game/Blueprints/Boss/BP_PlayerController_BossTest.BP_PlayerController_BossTest_C"))
    (for _array_element _outactors_2
      (`/Game/Blueprints/Boss/BP_PlayerController_BossTest.Show GameOver UI` _array_element))
    (else
      (bind _outactors_3 (`GameplayStatics.GetAllActorsOfClass` "/Game/Blueprints/Boss/BP_PlayerController_BossTest.BP_PlayerController_BossTest_C"))
      (for _array_element_2 _outactors_3
        (`/Game/Blueprints/Boss/BP_PlayerController_BossTest.Say Something` _array_element_2)))))

(fn `UserConstructionScript`)