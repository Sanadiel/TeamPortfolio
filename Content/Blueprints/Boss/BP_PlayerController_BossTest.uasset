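; BP_PlayerController_BossTest is a test player controller for the boss mode that shows game-over screens on the local player's machine.
; ShowGameOverUI branches on authority: the authority side gets the boss-lose widget, while remote clients get the player-win widget and a debug print.
; It only handles the boss-defeated outcome, with no opposite result.
; SaySomething prints the controlled pawn's name as a local debug message.
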(event `Say Something`
  (if (`self.IsLocalPlayerController`)
    (`KismetSystemLibrary.PrintString` (`KismetStringLibrary.Concat_StrStr` (`KismetSystemLibrary.GetDisplayName` (`self.K2_GetPawn`)) " Said!"))))

(event `Show GameOver UI`
  (if (`self.IsLocalPlayerController`)
    (`/Engine/EditorBlueprintResources/ActorMacros.Switch Has Authority`
      (:`Authority`
        (bind _returnvalue (`|CreateWidget` "/Game/Blueprints/Boss/BPforTest/WG_GameLose_Boss.WG_GameLose_Boss_C"))
        (`UserWidget.AddToViewport` _returnvalue 0))
      (:`Remote`
        (bind _returnvalue_2 (`|CreateWidget` "/Game/Blueprints/Boss/BPforTest/WG_GameWin_Player.WG_GameWin_Player_C"))
        (`UserWidget.AddToViewport` _returnvalue_2 0)
        (`KismetSystemLibrary.PrintString` "Remote In Player Controller")))))

(fn `UserConstructionScript`)