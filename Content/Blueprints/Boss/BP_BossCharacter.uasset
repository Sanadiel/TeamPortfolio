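; Boss character Blueprint that lets a locally controlled player click on widgets with a crosshair.
; On possession by a local controller, it creates the temporary crosshair widget and adds it to the viewport.
; The ButtonClick action forwards press and release to the WidgetInteraction component as left mouse button events, only on the locally controlled pawn.
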(event `self.ReceivePossessed`
  (params (NewController :type "Controller Object Reference"))
  (if (`Controller.IsLocalController` NewController)
    (bind _returnvalue (`|CreateWidget` "/Game/Blueprints/Boss/BPforTest/WG_TempCrossHair.WG_TempCrossHair_C"))
    (`UserWidget.AddToViewport` _returnvalue 0)))

(event `InputAction|ButtonClick`
  (params (Key :type "Key Structure"))
  (bind _widgetinteraction (`self.WidgetInteraction`))
  (:`Pressed`
    (if (`self.IsLocallyControlled`)
      (`WidgetInteractionComponent.PressPointerKey` _widgetinteraction "LeftMouseButton")))
  (:`Released`
    (if (`self.IsLocallyControlled`)
      (`WidgetInteractionComponent.ReleasePointerKey` _widgetinteraction "LeftMouseButton"))))

(fn `UserConstructionScript`)