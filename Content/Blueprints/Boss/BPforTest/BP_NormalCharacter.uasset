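; BP_NormalCharacter is a test player character for boss testing that fires projectiles and takes damage.
; The Fire input calls FireProjectile, which on authority spawns BP_NormalProjectile at SpawnPosition and plays a fire montage.
; Locally controlled instances add an HP_Test widget at BeginPlay, and AnyDamage subtracts from HP and prints the new value.
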(event `InputAction|Fire`
  (params (Key :type "Key Structure"))
  (:`Pressed`
    (`self.Fire Projectile`)))

(event `Fire Projectile`
  (`/Engine/EditorBlueprintResources/ActorMacros.Switch Has Authority`
    (:`Authority`
      (`|SpawnActorFromClass` "/Game/Blueprints/Boss/BPforTest/BP_NormalProjectile.BP_NormalProjectile_C" (`SceneComponent.K2_GetComponentToWorld` (`self.SpawnPosition`)) "Undefined" "OverrideRootScale" null null)
      (`self.PlayAnimMontage` (`self.FireAnimation`) 1.0 "Default"))))

(event `self.ReceiveBeginPlay`
  (if (`self.IsLocallyControlled`)
    (bind _returnvalue (`|CreateWidget` "/Game/Blueprints/Boss/BPforTest/HP_Test.HP_Test_C"))
    (`UserWidget.AddToViewport` _returnvalue 0)))

(event `self.ReceiveAnyDamage`
  (params (Damage :type "Float (single-precision)") (DamageType :type "DamageType Object Reference") (InstigatedBy :type "Controller Object Reference") (DamageCauser :type "Actor Object Reference"))
  (bind _output_get (set `self.HP` (- (`self.HP`) Damage)))
  (`KismetSystemLibrary.PrintString` (`KismetStringLibrary.Concat_StrStr` (`KismetSystemLibrary.GetDisplayName` self) " HP : " (`KismetStringLibrary.Conv_DoubleToString` _output_get))))

(fn `UserConstructionScript`)