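; BP_ThrowingSpawner is a spawner in the boss test folder that periodically spawns random throwing projectiles around itself.
; A looping timer counts MonsterSpawnProjectile actors in the world and, below MaxCount and only with authority, spawns a random class from ProjectileArray.
; Each spawn gets a random rotation and an X/Y offset bounded by the Sphere radius.
; The Sphere's world Z is added to the actor's location as the height offset.
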(event `self.ReceiveBeginPlay`
  (`KismetSystemLibrary.K2_SetTimerDelegate` (delegate `spawn`) (`self.SpawnFrequency`) true))

(event `spawn`
  (bind _projectilearray (`self.ProjectileArray`))
  (bind _sphere (`self.Sphere`))
  (bind _sphereradius (`SphereComponent.SphereRadius` _sphere))
  (bind _returnvalue (* -1 _sphereradius))
  (bind _outactors (`GameplayStatics.GetAllActorsOfClass` "/Script/TeamPortfolio.MonsterSpawnProjectile"))
  (if (< (`KismetArrayLibrary.Array_Length` _outactors) (`self.MaxCount`))
    (`/Engine/EditorBlueprintResources/ActorMacros.Switch Has Authority`
      (:`Authority`
        (`|SpawnActorFromClass` (`|GetArrayItem` _projectilearray (`KismetMathLibrary.RandomIntegerInRange` 0 (`KismetArrayLibrary.Array_LastIndex` _projectilearray))) (`KismetMathLibrary.MakeTransform` (+ (`self.K2_GetActorLocation`) (`KismetMathLibrary.MakeVector` (`KismetMathLibrary.RandomFloatInRange` _returnvalue _sphereradius) (`KismetMathLibrary.RandomFloatInRange` _returnvalue _sphereradius) (.z (`SceneComponent.GetSocketLocation` _sphere "None")))) (`KismetMathLibrary.RandomRotator` false)) "Undefined" "OverrideRootScale" null null)))))

(fn `UserConstructionScript`)