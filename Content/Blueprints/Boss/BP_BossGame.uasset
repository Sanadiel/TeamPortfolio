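; BP_BossGame tracks the objectives in a boss match and detects the normal players' win.
; On BeginPlay it caches all BP_ObjectiveActor instances and binds a handler to the WhenObjectiveDestroyed event.
; On each destruction, the authority re-queries the remaining objectives and, when none are left, only prints a win message.
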(event `self.ReceiveBeginPlay`
  (bind _outactors (`GameplayStatics.GetAllActorsOfClass` "/Game/Blueprints/Boss/BPforTest/BP_ObjectiveActor.BP_ObjectiveActor_C"))
  (set `self.ObjectiveActorArray` _outactors)
  (add `self.WhenObjectiveDestroyed` (delegate `OnObjectiveDestroyed`)))

(event `OnObjectiveDestroyed`
  (`/Engine/EditorBlueprintResources/ActorMacros.Switch Has Authority`
    (:`Authority`
      (bind _outactors (`GameplayStatics.GetAllActorsOfClass` "/Game/Blueprints/Boss/BPforTest/BP_ObjectiveActor.BP_ObjectiveActor_C"))
      (bind _output_get (set `self.ObjectiveActorArray` _outactors))
      (if (<= (`KismetArrayLibrary.Array_Length` _output_get) 0)
        (`KismetSystemLibrary.PrintString` "Normal Player Win!")))))

(fn `UserConstructionScript`)