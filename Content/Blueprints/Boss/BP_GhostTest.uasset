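; BP_GhostTest is a possessable test Blueprint that clicks widgets through a WidgetInteraction component.
; BeginPlay enables orientation tracking and checks for a connected headset, adding a temporary crosshair widget when none is found.
; ButtonClick press and release drive the left mouse pointer key on that component, only when locally controlled.
; The construction script and UI-visibility RepNotify are empty, and the Possessed local-controller check leads nowhere.
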(event `self.ReceiveBeginPlay`
  (`parent.ReceiveBeginPlay`)
  (`OculusFunctionLibrary.EnableOrientationTracking` true)
  (if (not (`HeadMountedDisplayFunctionLibrary.IsHeadMountedDisplayConnected`))
    (`KismetSystemLibrary.PrintString` "Not VR")
    (bind _returnvalue (`|CreateWidget` "/Game/Blueprints/Boss/BPforTest/WG_TempCrossHair.WG_TempCrossHair_C"))
    (`UserWidget.AddToViewport` _returnvalue 0)
    (else
      (`KismetSystemLibrary.PrintString` "VR Mode"))))

(event `self.ReceivePossessed`
  (params (NewController :type "Controller Object Reference"))
  (`parent.ReceivePossessed` NewController)
  (if (`Controller.IsLocalPlayerController` NewController)
    _))

(event `InputAction|ButtonClick`
  (params (Key :type "Key Structure"))
  (:`Pressed`
    (if (`self.IsLocallyControlled`)
      (`WidgetInteractionComponent.PressPointerKey` (`self.WidgetInteraction`) "LeftMouseButton")))
  (:`Released`
    (if (`self.IsLocallyControlled`)
      (`WidgetInteractionComponent.ReleasePointerKey` (`self.WidgetInteraction`) "LeftMouseButton"))))

(fn `OnRep_UI See`)

(fn `UserConstructionScript`)