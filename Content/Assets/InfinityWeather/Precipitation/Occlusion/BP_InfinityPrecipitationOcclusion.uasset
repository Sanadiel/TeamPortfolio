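; Placeable actor that captures an orthographic height map of a square area for precipitation occlusion in the Infinity Weather system.
; Initialize publishes its location and AreaSize to MPC_InfinityWeather, sizes the preview box, plane and SceneCapture2D, and applies render filters.
; It runs at construction and BeginPlay, which then destroys the preview components and calls CaptureScene once after CaptureDelay.
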(event `self.ReceiveBeginPlay`
  (`self.Initialize`)
  (`self.EditorOnly`)
  (`KismetSystemLibrary.Delay` (`self.CaptureDelay`))
  (`SceneCaptureComponent2D.CaptureScene` (`self.SceneCaptureComponent2D`)))

(fn `EditorOnly`
  (`|ExecutionSequence`
    (:`then_0`
      (`/Engine/EditorBlueprintResources/StandardMacros.IsValid` (`self.Plane`)
        (:`Is Valid`
          (`SceneComponent.SetVisibility` (`self.Plane`) (`self.EditorPreview`) false)
          (`ActorComponent.K2_DestroyComponent` (`self.Plane`)))))
    (:`then_1`
      (`/Engine/EditorBlueprintResources/StandardMacros.IsValid` (`self.Box`)
        (:`Is Valid`
          (`ActorComponent.K2_DestroyComponent` (`self.Box`)))))))

(fn `Initialize`
  (bind (_returnvalue_x _returnvalue_y _returnvalue_z) (`KismetMathLibrary.BreakVector` (`self.K2_GetActorLocation`)))
  (bind _scenecapturecomponent2d (`self.SceneCaptureComponent2D`))
  (bind _box (`self.Box`))
  (bind _returnvalue (/ (`self.AreaSize`) 100.0))
  (bind _returnvalue_2 (* (`self.AreaSize`) 0.5))
  (`|ExecutionSequence`
    (:`then_0`
      (`KismetMaterialLibrary.SetVectorParameterValue` "/Game/Assets/InfinityWeather/MPC_InfinityWeather.MPC_InfinityWeather" "HeightMapLocation" (make `LinearColor` _returnvalue_x _returnvalue_y _returnvalue_z (`self.AreaSize`))))
    (:`then_1`
      (`/Engine/EditorBlueprintResources/StandardMacros.IsValid` _box
        (:`Is Valid`
          (`BoxComponent.SetBoxExtent` _box (`KismetMathLibrary.MakeVector` _returnvalue_2 _returnvalue_2) true))))
    (:`then_2`
      (`/Engine/EditorBlueprintResources/StandardMacros.IsValid` (`self.Plane`)
        (:`Is Valid`
          (`SceneComponent.SetWorldScale3D` (`self.Plane`) (`KismetMathLibrary.MakeVector` _returnvalue _returnvalue _returnvalue)))))
    (:`then_3`
      (set `SceneCaptureComponent2D.OrthoWidth` (`self.AreaSize`) _scenecapturecomponent2d)
      (set `SceneCaptureComponent.PrimitiveRenderMode` (`self.PrimitiveRender`) _scenecapturecomponent2d)
      (set `SceneCaptureComponent.HiddenActors` (`self.HiddenActors`) (`self.SceneCaptureComponent2D`))
      (set `SceneCaptureComponent.ShowOnlyActors` (`self.ShowOnlyActors`) (`self.SceneCaptureComponent2D`)))
    (:`then_4`
      (`SceneComponent.SetVisibility` (`self.Plane`) (`self.EditorPreview`) false)
      (`SceneComponent.SetHiddenInGame` (`self.Plane`) (`self.HiddenInGame`) false))))

(fn `UserConstructionScript`
  (`self.Initialize`))