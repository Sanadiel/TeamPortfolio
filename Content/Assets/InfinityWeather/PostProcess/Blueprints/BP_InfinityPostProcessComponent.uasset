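; Camera component that drives InfinityWeather screen effects: raindrops, frost, sharpening, air distortion and glittering.
; A looping timer samples precipitation and atmosphere from BP_InfinityWeatherController at the camera and line-traces against precipitation for occlusion.
; Tick eases screen wetness and ice over time.
; Active effects form bitmasks indexing prebuilt material permutations, keeping one post-process and one pre-translucent blendable on the camera.
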(event `self.ReceiveBeginPlay`
  (`KismetArrayLibrary.Array_Clear` (`self.PostProcessInstances`))
  (`KismetArrayLibrary.Array_Clear` (`self.PreTranslucentInstances`))
  (`/Engine/EditorBlueprintResources/StandardMacros.IsValid` (`self.PostProcessCamera`)
    (:`Is Valid`
      _)
    (:`Is Not Valid`
      (set `self.PostProcessCamera` (`Actor.GetComponentByClass` (`self.GetOwner`) "/Script/Engine.CameraComponent"))))
  (`self.SetEnabled` (`self.IsActive`)))

(event `self.ReceiveTick`
  (params (DeltaSeconds :type "Float (single-precision)"))
  (if (`self.IsActive`)
    (`self.Update` DeltaSeconds)))

(event `self.ReceiveEndPlay`
  (params (EndPlayReason :type "EEndPlayReason Enum" :default "Destroyed"))
  (`self.SetEnabled` false))

(fn `SetEnabled`
  (params (Enabled :type Boolean))
  (bind _returnvalue (`KismetSystemLibrary.K2_IsTimerActive` null "UpdateData"))
  (if Enabled
    (if (not _returnvalue)
      (`|ExecutionSequence`
        (:`then_0`
          ;[1 1 1] Init
          (`KismetSystemLibrary.K2_SetTimer` null "UpdateData" (`self.UpdateDataFrequency`) true)
          (`self.SetPostprocess` 0)
          (`self.SetPreTranslucent` 0)
          (bind _returnvalue_2 (`GameplayStatics.GetActorOfClass` "/Game/Assets/InfinityWeather/Weather/Blueprints/BP_InfinityWeatherController.BP_InfinityWeatherController_C"))
          (bind _output_get (set `self.Controller` _returnvalue_2))
          (`/Engine/EditorBlueprintResources/StandardMacros.IsValid` _output_get))
        (:`then_1`
          ;[1 1 1] Create material permutations
          (if (== (`KismetArrayLibrary.Array_Length` (`self.PostProcessInstances`)) 0)
            (for (_array_element _array_index) (`self.PostprocessMaterials`)
              (bind _returnvalue_3 (`KismetMaterialLibrary.CreateDynamicMaterialInstance` _array_element))
              (`KismetArrayLibrary.Array_Set` (`self.PostProcessInstances`) _array_index _returnvalue_3 true))))
        (:`then_2`
          (if (== (`KismetArrayLibrary.Array_Length` (`self.PreTranslucentInstances`)) 0)
            (for (_array_element_2 _array_index_2) (`self.PreTranslucentMaterials`)
              (bind _returnvalue_4 (`KismetMaterialLibrary.CreateDynamicMaterialInstance` _array_element_2))
              (`KismetArrayLibrary.Array_Set` (`self.PreTranslucentInstances`) _array_index_2 _returnvalue_4 true))))))
    (elif _returnvalue
      ;[1 1 1] Remove
      (`self.SetPostprocess` 0)
      (`self.SetPreTranslucent` 0)
      (`KismetSystemLibrary.K2_ClearTimer` null "UpdateData")
      (`/Engine/EditorBlueprintResources/StandardMacros.IsValid` (`self.Controller`)))))

(fn `SetPostprocess`
  (params (Effect :type Integer))
  (if (!= Effect (`self.CurrentPostprocess`))
    (`CameraComponent.RemoveBlendable` (`self.PostProcessCamera`) (`self.PostProcesInstance`))
    (set `self.CurrentPostprocess` (`local.Effect`))
    (bind _output_get (set `self.PostProcesInstance` (`|GetArrayItem` (`self.PostProcessInstances`) (`self.CurrentPostprocess`))))
    (`CameraComponent.AddOrUpdateBlendable` (`self.PostProcessCamera`) _output_get 1.0)))

(fn `SetPreTranslucent`
  (params (Effect :type Integer))
  (if (!= Effect (`self.CurrentPreTranslucent`))
    (`CameraComponent.RemoveBlendable` (`self.PostProcessCamera`) (`self.PreTranslucentInstance`))
    (set `self.CurrentPreTranslucent` (`local.Effect`))
    (bind _output_get (set `self.PreTranslucentInstance` (`|GetArrayItem` (`self.PreTranslucentInstances`) (`self.CurrentPreTranslucent`))))
    (`CameraComponent.AddOrUpdateBlendable` (`self.PostProcessCamera`) _output_get 1.0)))

(fn `SetScreenRainSplash`
  (params (RainIntensity :type "Float (double-precision)"))
  (set `self.RainDropsOnScreen` (`KismetMathLibrary.FMax` (`local.RainIntensity`) (`self.RainDropsOnScreen`))))

(fn `Update`
  (params (DeltaTime :type "Float (double-precision)"))
  (locals (FinalPostprocess :type Integer) (NewLocalVar_0 :type Integer :default 0))
  (`self.UpdateFeezing` (`local.DeltaTime`))
  (`self.UpdateRain` (`local.DeltaTime`))
  (`self.UpdatePostProcess`)
  (`self.UpdatePreTranslucent`))

(fn `UpdateData`
  (locals (CameraLocation :type "Vector Structure" :default (0.0 0.0 0.0)) (CameraForward :type "Vector Structure" :default (0.0 0.0 0.0)))
  (bind _postprocesscamera (`self.PostProcessCamera`))
  (bind _cameralocation (`local.CameraLocation`))
  (`/Engine/EditorBlueprintResources/StandardMacros.IsValid` (`self.Controller`)
    (:`Is Valid`
      (set `local.CameraLocation` (`SceneComponent.K2_GetComponentLocation` _postprocesscamera))
      (set `local.CameraForward` (`SceneComponent.GetForwardVector` _postprocesscamera))
      (`|ExecutionSequence`
        (:`then_0`
          (bind (_rain _snow _wind _force) (`/Game/Assets/InfinityWeather/Weather/Blueprints/BP_InfinityWeatherController.GetPrecipitationDataAtLocation` (`self.Controller`) (`local.CameraLocation`)))
          (set `self.RainIntensity` _rain)
          (set `self.SnowIntensity` _snow)
          (set `self.WindIntensity` _wind)
          (set `self.PrecipitationForce` _force)
          (if (`self.UseOcclusionUpDirection`)
            (set `self.PrecipitationForce` (0.0 0.0 -1.0))))
        (:`then_1`
          (bind _data (`/Game/Assets/InfinityWeather/Weather/Blueprints/BP_InfinityWeatherController.GetAtmosphereDataAtLocation` (`self.Controller`) (`local.CameraLocation`)))
          (set `self.AirDistortion` (`.Distortion_57_DD466BA345F7D1633FAF138599D9A41B` (break `/Game/Assets/InfinityWeather/Environment/Fog/BS_InfinityAtmosphere` _data)))
          (set `self.AirHumidity` (`.Humidity_58_5C8EA7B14FB334B29B150081DD9EF43E` (break `/Game/Assets/InfinityWeather/Environment/Fog/BS_InfinityAtmosphere` _data)))
          (set `self.AirTemperature` (`.Temperature_59_CE6ED57F4C130C870740B288A8FC2A36` (break `/Game/Assets/InfinityWeather/Environment/Fog/BS_InfinityAtmosphere` _data))))
        (:`then_2`
          (if (and (<= (`self.RainIntensity`) 0.0) (<= (`self.RainIntensity`) 0.0))
            (set `self.IsOccluded` true :!label _label)
            (elif (< (* (`KismetMathLibrary.Dot_VectorVector` (`local.CameraForward`) (`self.PrecipitationForce`)) -1.0) (`self.OcclustionAngleTest`))
              (goto _label)
              (else
                (bind (_outhit _returnvalue) (`KismetSystemLibrary.LineTraceSingle` _cameralocation (- _cameralocation (* (`self.PrecipitationForce`) (`self.OcclusionDistanceTest`))) "TraceTypeQuery2" false (`|MakeArray` (`self.GetOwner`))))
                (set `self.IsOccluded` _returnvalue)))))))))

(fn `UpdateFeezing`
  (params (DeltaTime :type "Float (double-precision)"))
  (locals (MaxFrozen :type "Float (double-precision)"))
  (if (not (and (>= (`self.ScreenIce`) -0.02) (>= (`self.AirTemperature`) 0.0)))
    (bind _output_get (set `self.ScreenTemperature` (`KismetMathLibrary.Lerp` (`self.ScreenTemperature`) (`self.AirTemperature`) (* (`local.DeltaTime`) (`self.AirBlendSpeed`)))))
    (set `local.MaxFrozen` (`CurveFloat.GetFloatValue` (`self.MaxFrozenOverTemperature`) _output_get))
    (set `self.ScreenIce` (select `bool` (< (`local.MaxFrozen`) (`self.ScreenIce`)) :`false` (`KismetMathLibrary.FMin` (+ (`self.ScreenIce`) (* (`local.DeltaTime`) (`self.IceMeltingSpeed`) (`KismetMathLibrary.FMax` (`self.ScreenTemperature`) 1.0))) (`local.MaxFrozen`)) :`true` (`KismetMathLibrary.FClamp` (+ (`self.ScreenIce`) (* (`self.ScreenTemperature`) (`self.AirHumidity`) (`self.FreezingSpeed`) (`local.DeltaTime`))) (`local.MaxFrozen`))))))

(fn `UpdatePostProcess`
  (locals (FinalMask :type Integer :default 0))
  (if (> (`self.UsePostProcess`) 0)
    (set `local.FinalMask` 0)
    (`|ExecutionSequence`
      (:`then_0`
        (if (> (`self.SharpenIntensity`) 0.0)
          (set `local.FinalMask` (`KismetMathLibrary.Or_IntInt` (`local.FinalMask`) (`|BitmaskLiteral` 4)))))
      (:`then_1`
        (if (> (`self.RainDropsOnScreen`) 0.0)
          (set `local.FinalMask` (`KismetMathLibrary.Or_IntInt` (`local.FinalMask`) (`|BitmaskLiteral` 1)))))
      (:`then_2`
        (if (< (`self.ScreenIce`) 0.0)
          (set `local.FinalMask` (`KismetMathLibrary.Or_IntInt` (`local.FinalMask`) (`|BitmaskLiteral` 2)))))
      (:`then_3`
        (`self.SetPostprocess` (`KismetMathLibrary.And_IntInt` (`local.FinalMask`) (`self.UsePostProcess`)))
        (if (> (`self.CurrentPostprocess`) 0)
          (`|ExecutionSequence`
            (:`then_0`
              (if (> (`KismetMathLibrary.And_IntInt` (`self.CurrentPostprocess`) (`|BitmaskLiteral` 1)) 0)
                (`MaterialInstanceDynamic.SetScalarParameterValue` (`self.PostProcesInstance`) "RaindropsShow" (`self.RainDropsOnScreen`))
                (`MaterialInstanceDynamic.SetScalarParameterValue` (`self.PostProcesInstance`) "AnimationTimeOffset" (`self.RaindropsTime`))))
            (:`then_1`
              (if (> (`KismetMathLibrary.And_IntInt` (`self.CurrentPostprocess`) (`|BitmaskLiteral` 4)) 0)
                (`MaterialInstanceDynamic.SetScalarParameterValue` (`self.PostProcesInstance`) "SharpenFade" (`self.SharpenIntensity`))))
            (:`then_2`
              (if (> (`KismetMathLibrary.And_IntInt` (`self.CurrentPostprocess`) (`|BitmaskLiteral` 2)) 0)
                (`MaterialInstanceDynamic.SetVectorParameterValue` (`self.PostProcesInstance`) "FrozenScale" (* (- (`CurveLinearColor.GetLinearColorValue` (`self.FreezingAnimation`) (* (`self.ScreenIce`) -1.0)) (struct :`R` 0.5 :`G` 0.5 :`B` 0.5 :`A` 0.5)) 5.0))))))))
    (else
      (`self.SetPostprocess` (`self.UsePostProcess`)))))

(fn `UpdatePreTranslucent`
  (locals (FinalMask :type Integer :default 0))
  (if (> (`self.UsePreTranslucent`) 0)
    (set `local.FinalMask` 0)
    (`|ExecutionSequence`
      (:`then_0`
        ;[1 1 1] Build bitmask
        (if (> (`self.RainIntensity`) 0.0)
          (set `local.FinalMask` (`KismetMathLibrary.Or_IntInt` (`local.FinalMask`) (`|BitmaskLiteral` 1)))))
      (:`then_1`
        (if (> (`self.AirDistortion`) 0.0)
          (set `local.FinalMask` (`KismetMathLibrary.Or_IntInt` (`local.FinalMask`) (`|BitmaskLiteral` 2)))))
      (:`then_2`
        (if (> (`self.GlitteringIntensity`) 0.0)
          (set `local.FinalMask` (`KismetMathLibrary.Or_IntInt` (`local.FinalMask`) (`|BitmaskLiteral` 4)))))
      (:`then_3`
        ;[1 1 1] Update parameters
        (`self.SetPreTranslucent` (`KismetMathLibrary.And_IntInt` (`local.FinalMask`) (`self.UsePreTranslucent`)))
        (if (> (`self.CurrentPreTranslucent`) 0)
          (`|ExecutionSequence`
            (:`then_0`
              (if (> (`KismetMathLibrary.And_IntInt` (`self.CurrentPreTranslucent`) (`|BitmaskLiteral` 1)) 0)
                (`MaterialInstanceDynamic.SetScalarParameterValue` (`self.PreTranslucentInstance`) "RaindropsShow" (`self.RainIntensity`))))
            (:`then_1`
              (if (> (`KismetMathLibrary.And_IntInt` (`self.CurrentPreTranslucent`) (`|BitmaskLiteral` 2)) 0)
                (`MaterialInstanceDynamic.SetScalarParameterValue` (`self.PreTranslucentInstance`) "DistortionShow" (`self.AirDistortion`))))
            (:`then_2`
              (if (> (`KismetMathLibrary.And_IntInt` (`self.CurrentPreTranslucent`) (`|BitmaskLiteral` 4)) 0)
                (`MaterialInstanceDynamic.SetScalarParameterValue` (`self.PreTranslucentInstance`) "GlitteringShow" (`self.GlitteringIntensity`))))))))
    (else
      (`self.SetPreTranslucent` (`self.UsePreTranslucent`)))))

(fn `UpdateRain`
  (params (DeltaTime :type "Float (double-precision)"))
  (if (or (`self.IsOccluded`) (<= (`self.RainIntensity`) 0.0))
    (set `self.RainDropsOnScreen` (`KismetMathLibrary.FInterpTo_Constant` (`self.RainDropsOnScreen`) 0.0 (`local.DeltaTime`) (`self.DryingSpeed`)))
    (else
      (set `self.RaindropsTime` (+ (`self.RaindropsTime`) (* (`local.DeltaTime`) (`self.RaindropsAnimSpeed`))))
      (set `self.RainDropsOnScreen` (`KismetMathLibrary.FInterpTo_Constant` (`self.RainDropsOnScreen`) (`self.RainIntensity`) (`local.DeltaTime`) (select `bool` (> (`self.RainIntensity`) (`self.RainDropsOnScreen`)) :`false` (`self.DryingSpeed`) :`true` (`self.GettingWetSpeed`)))))))