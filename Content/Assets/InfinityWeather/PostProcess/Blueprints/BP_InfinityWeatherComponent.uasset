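; Camera post-process weather component for Infinity Weather, driving screen raindrops, frost and air distortion, plus an optional breath emitter in freezing air.
; It adds two dynamic materials as camera blendables and registers with the weather controller.
; A looping timer samples precipitation and fog at the camera and line-traces against precipitation direction for occlusion.
; Tick interpolates wetting and drying, and derives screen ice from temperature and humidity through curves.
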(event `self.ReceiveBeginPlay`
  (set `self.PostProcessCamera` (`Actor.GetComponentByClass` (`self.GetOwner`) "/Script/Engine.CameraComponent"))
  (`self.SetEnabled` (`self.IsActive`)))

(event `self.ReceiveTick`
  (params (DeltaSeconds :type "Float (single-precision)"))
  (if (`self.IsActive`)
    (`self.Update` DeltaSeconds)))

(event `self.ReceiveEndPlay`
  (params (EndPlayReason :type "EEndPlayReason Enum" :default "Destroyed"))
  (`self.SetEnabled` false))

(fn `SetEnabled`
  (params (Enabled :type Boolean))
  (bind _controller (`self.Controller`))
  (if Enabled
    (`/Engine/EditorBlueprintResources/StandardMacros.IsValid` (`self.PreTranslucentInstance`)
      (:`Is Not Valid`
        ;[1 1 1] Init
        (`|ExecutionSequence`
          (:`then_0`
            (bind _returnvalue (`KismetMaterialLibrary.CreateDynamicMaterialInstance` "/Game/Assets/InfinityWeather/PostProcess/Materials/MI_InfinityPreTranslucent.MI_InfinityPreTranslucent"))
            (set `self.PreTranslucentInstance` _returnvalue)
            (`CameraComponent.AddOrUpdateBlendable` (`self.PostProcessCamera`) (`self.PreTranslucentInstance`) 1.0))
          (:`then_1`
            (bind _returnvalue_2 (`KismetMaterialLibrary.CreateDynamicMaterialInstance` "/Game/Assets/InfinityWeather/PostProcess/Materials/MI_InfinityPostProcess.MI_InfinityPostProcess"))
            (set `self.PostProcesInstance` _returnvalue_2)
            (`CameraComponent.AddOrUpdateBlendable` (`self.PostProcessCamera`) (`self.PostProcesInstance`) 1.0))
          (:`then_2`
            (bind _returnvalue_3 (`GameplayStatics.GetActorOfClass` "/Game/Assets/InfinityWeather/BP_InfinityWeatherController.BP_InfinityWeatherController_C"))
            (bind _output_get (set `self.Controller` _returnvalue_3))
            (`/Engine/EditorBlueprintResources/StandardMacros.IsValid` _output_get
              (:`Is Valid`
                (`/Game/Assets/InfinityWeather/BP_InfinityWeatherController.AddPostProcessComponent` _output_get self))))
          (:`then_3`
            (`self.UpdateFeezing` 0.0))
          (:`then_4`
            (`KismetSystemLibrary.K2_SetTimer` null "UpdateData" (`self.UpdateDataFrequency`) true)))))
    (else
      ;[1 1 1] Remove
      (`|ExecutionSequence`
        (:`then_0`
          (`/Engine/EditorBlueprintResources/StandardMacros.IsValid` (`self.PreTranslucentInstance`)
            (:`Is Valid`
              (`CameraComponent.RemoveBlendable` (`self.PostProcessCamera`) (`self.PreTranslucentInstance`))
              (set `self.PostProcesInstance` (`self.PreTranslucentInstance`)))))
        (:`then_1`
          (`/Engine/EditorBlueprintResources/StandardMacros.IsValid` (`self.PostProcesInstance`)
            (:`Is Valid`
              (`CameraComponent.RemoveBlendable` (`self.PostProcessCamera`) (`self.PostProcesInstance`))
              (set `self.PostProcesInstance` null))))
        (:`then_2`
          (`/Engine/EditorBlueprintResources/StandardMacros.IsValid` _controller
            (:`Is Valid`
              (`KismetArrayLibrary.Array_RemoveItem` (`/Game/Assets/InfinityWeather/BP_InfinityWeatherController.PostProcessComponents` _controller) self))))
        (:`then_3`
          (`KismetSystemLibrary.K2_ClearTimer` null "UpdateData"))))))

(fn `SetOwnerBreathe`
  (params (Enable :type Boolean) (Mesh :type "SkeletalMeshComponent Object Reference"))
  (bind (_breatheffecttransform_location _breatheffecttransform_rotation _breatheffecttransform_scale) (`KismetMathLibrary.BreakTransform` (`self.BreathEffectTransform`)))
  (if Enable
    (if (and (`self.IsActive`) (`self.UseBreath`))
      (if (< (`self.AirTemperature`) 0.0)
        (`/Engine/EditorBlueprintResources/StandardMacros.IsValid` (`self.SpawnedBretheEffect`)
          (:`Is Not Valid`
            (bind _returnvalue (`GameplayStatics.SpawnEmitterAttached` (`self.BreathEffect`) (`local.Mesh`) (`self.BreathEffectAttachement`) _breatheffecttransform_location _breatheffecttransform_rotation _breatheffecttransform_scale "KeepRelativeOffset" false "AutoRelease"))
            (set `self.SpawnedBretheEffect` _returnvalue)))))
    (else
      (`/Engine/EditorBlueprintResources/StandardMacros.IsValid` (`self.SpawnedBretheEffect`)
        (:`Is Valid`
          (`self.Deactivate` (`self.SpawnedBretheEffect`))
          (set `self.SpawnedBretheEffect` null))))))

(fn `SetScreenRainSplash`
  (params (RainIntensity :type "Float (double-precision)"))
  (set `self.RainDropsOnScreen` (`KismetMathLibrary.FMax` (`local.RainIntensity`) (`self.RainDropsOnScreen`))))

(fn `Update`
  (params (DeltaTime :type "Float (double-precision)"))
  (locals (MaxFrozen :type "Float (double-precision)" :default 0.0))
  (`|ExecutionSequence`
    (:`then_0`
      ;[1 1 1] Rain falling on screen
      (if (or (`self.IsOccluded`) (<= (`self.RainIntensity`) 0.0))
        (set `self.RainDropsOnScreen` (`KismetMathLibrary.FInterpTo_Constant` (`self.RainDropsOnScreen`) 0.0 (`local.DeltaTime`) (`self.DryingSpeed`)))
        (else
          (set `self.RaindropsTime` (+ (`self.RaindropsTime`) (* (`local.DeltaTime`) (`self.RaindropsAnimSpeed`))))
          (set `self.RainDropsOnScreen` (`KismetMathLibrary.FInterpTo_Constant` (`self.RainDropsOnScreen`) (`self.RainIntensity`) (`local.DeltaTime`) (select `bool` (> (`self.RainIntensity`) (`self.RainDropsOnScreen`)) :`false` (`self.DryingSpeed`) :`true` (`self.GettingWetSpeed`))))
          (`MaterialInstanceDynamic.SetScalarParameterValue` (`self.PostProcesInstance`) "AnimationTimeOffset" (`self.RaindropsTime`)))))
    (:`then_1`
      (if (> (`self.RainDropsOnScreen`) 0.0)
        (`MaterialInstanceDynamic.SetScalarParameterValue` (`self.PostProcesInstance`) "RaindropsShow" (`self.RainDropsOnScreen`))))
    (:`then_2`
      (`MaterialInstanceDynamic.SetScalarParameterValue` (`self.PreTranslucentInstance`) "RaindropsShow" (`self.RainIntensity`)))
    (:`then_3`
      (if (not (and (>= (`self.ScreenIce`) -0.02) (>= (`self.AirTemperature`) 0.0)))
        (`self.UpdateFeezing` (`local.DeltaTime`))))
    (:`then_4`
      (`MaterialInstanceDynamic.SetScalarParameterValue` (`self.PreTranslucentInstance`) "DistortionShow" (`self.AirDistortion`)))))

(fn `UpdateData`
  (locals (CameraLocation :type "Vector Structure" :default (0.0 0.0 0.0)) (CameraForward :type "Vector Structure" :default (0.0 0.0 0.0)))
  (bind _postprocesscamera (`self.PostProcessCamera`))
  (bind _cameralocation (`local.CameraLocation`))
  (`/Engine/EditorBlueprintResources/StandardMacros.IsValid` (`self.Controller`)
    (:`Is Valid`
      (set `local.CameraLocation` (`SceneComponent.K2_GetComponentLocation` _postprocesscamera))
      (set `local.CameraForward` (`SceneComponent.GetForwardVector` _postprocesscamera))
      (`|ExecutionSequence`
        (:`then_0`
          (bind (_rain _snow _wind _force) (`/Game/Assets/InfinityWeather/BP_InfinityWeatherController.GetPrecipitationDataAtLocation` (`self.Controller`) (`local.CameraLocation`)))
          (set `self.RainIntensity` _rain)
          (set `self.SnowIntensity` _snow)
          (set `self.WindIntensity` _wind)
          (set `self.PrecipitationForce` _force)
          (if (`self.UseOcclusionUpDirection`)
            (set `self.PrecipitationForce` (0.0 0.0 -1.0))))
        (:`then_1`
          (bind _data (`/Game/Assets/InfinityWeather/BP_InfinityWeatherController.GetFogDataAtLocation` (`self.Controller`) (`local.CameraLocation`)))
          (set `self.AirDistortion` (`.Distortion_57_DD466BA345F7D1633FAF138599D9A41B` (break `/Game/Assets/InfinityWeather/Environment/Fog/BS_InfinityAtmosphere` _data)))
          (set `self.AirHumidity` (`.Humidity_58_5C8EA7B14FB334B29B150081DD9EF43E` (break `/Game/Assets/InfinityWeather/Environment/Fog/BS_InfinityAtmosphere` _data)))
          (set `self.AirTemperature` (`.Temperature_59_CE6ED57F4C130C870740B288A8FC2A36` (break `/Game/Assets/InfinityWeather/Environment/Fog/BS_InfinityAtmosphere` _data))))
        (:`then_2`
          (if (and (<= (`self.RainIntensity`) 0.0) (<= (`self.RainIntensity`) 0.0))
            (set `self.IsOccluded` true :!label _label)
            (elif (< (* (`KismetMathLibrary.Dot_VectorVector` (`local.CameraForward`) (`self.PrecipitationForce`)) -1.0) (`self.OcclustionAngleTest`))
              (goto _label)
              (else
                (bind (_outhit _returnvalue) (`KismetSystemLibrary.LineTraceSingle` _cameralocation (- _cameralocation (* (`self.PrecipitationForce`) (`self.OcclusionDistanceTest`))) "TraceTypeQuery2" false (`|MakeArray` (`self.GetOwner`))))
                (set `self.IsOccluded` _returnvalue)))))))))

(fn `UpdateFeezing`
  (params (DeltaTime :type "Float (double-precision)"))
  (locals (MaxFrozen :type "Float (double-precision)"))
  (bind _output_get (set `self.ScreenTemperature` (`KismetMathLibrary.Lerp` (`self.ScreenTemperature`) (`self.AirTemperature`) (* (`local.DeltaTime`) (`self.AirBlendSpeed`)))))
  (set `local.MaxFrozen` (`CurveFloat.GetFloatValue` (`self.MaxFrozenOverTemperature`) _output_get))
  (set `self.ScreenIce` (select `bool` (< (`local.MaxFrozen`) (`self.ScreenIce`)) :`false` (`KismetMathLibrary.FMin` (+ (`self.ScreenIce`) (* (`local.DeltaTime`) (`self.IceMeltingSpeed`) (`KismetMathLibrary.FMax` (`self.ScreenTemperature`) 1.0))) (`local.MaxFrozen`)) :`true` (`KismetMathLibrary.FClamp` (+ (`self.ScreenIce`) (* (`self.ScreenTemperature`) (`self.AirHumidity`) (`self.FreezingSpeed`) (`local.DeltaTime`))) (`local.MaxFrozen`))))
  (`MaterialInstanceDynamic.SetVectorParameterValue` (`self.PostProcesInstance`) "FrozenScale" (* (- (`CurveLinearColor.GetLinearColorValue` (`self.FreezingAnimation`) (* (`self.ScreenIce`) -1.0)) (struct :`R` 0.5 :`G` 0.5 :`B` 0.5 :`A` 0.5)) 5.0)))