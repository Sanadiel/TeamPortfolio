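; BP_FootstepPreset is an InfinityWeather footstep preset that plays a particle effect and sound for a step.
; Spawn attaches the preset's Effect and Sound to the given mesh, using the bone and transform from the attachment struct.
; The sound uses the preset's volume, pitch and attenuation, and both spawned components are returned.
; The Intensity input is not used in Spawn.
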(fn `Spawn`
  (params (Mesh :type "SkeletalMeshComponent Object Reference") (Attachement :type "/Game/Assets/InfinityWeather/Footstep/Blueprints/BS_FootstepAttachement Structure") (Intensity :type "Float (double-precision)"))
  (returns (SpawnedAudio :type "AudioComponent Object Reference") (SpawnedEmitter :type "ParticleSystemComponent Object Reference"))
  (bind _attachement (`local.Attachement`))
  (bind _attachement_2 (`local.Attachement`))
  (bind _returnvalue (`GameplayStatics.SpawnEmitterAttached` (`self.Effect`) (`local.Mesh`) (break `/Game/Assets/InfinityWeather/Footstep/Blueprints/BS_FootstepAttachement` _attachement_2) (.location (`.Transform_5_8FCEC8CE48DEEB25B75579993D36D8AB` (break `/Game/Assets/InfinityWeather/Footstep/Blueprints/BS_FootstepAttachement` _attachement_2))) (.rotation (`.Transform_5_8FCEC8CE48DEEB25B75579993D36D8AB` (break `/Game/Assets/InfinityWeather/Footstep/Blueprints/BS_FootstepAttachement` _attachement_2))) (.scale (`.Transform_5_8FCEC8CE48DEEB25B75579993D36D8AB` (break `/Game/Assets/InfinityWeather/Footstep/Blueprints/BS_FootstepAttachement` _attachement_2)))))
  (bind _returnvalue_2 (`GameplayStatics.SpawnSoundAttached` (`self.Sound`) (`local.Mesh`) (break `/Game/Assets/InfinityWeather/Footstep/Blueprints/BS_FootstepAttachement` _attachement) (.location (`.Transform_5_8FCEC8CE48DEEB25B75579993D36D8AB` (break `/Game/Assets/InfinityWeather/Footstep/Blueprints/BS_FootstepAttachement` _attachement))) (.rotation (`.Transform_5_8FCEC8CE48DEEB25B75579993D36D8AB` (break `/Game/Assets/InfinityWeather/Footstep/Blueprints/BS_FootstepAttachement` _attachement))) "KeepRelativeOffset" false (`self.VolumeMultiplier`) (`self.PitchMultiplier`) 0.0 (`self.Attenuation`) null))
  (return _returnvalue_2 _returnvalue))