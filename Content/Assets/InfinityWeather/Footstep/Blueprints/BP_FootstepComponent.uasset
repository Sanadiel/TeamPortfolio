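; Footstep component that spawns surface-dependent effects at a mesh bone when Play is called.
; BeginPlay builds one instance per template; Play sphere-traces WorldStatic and picks the instance by physical surface type.
; The highest-priority active override volume replaces that choice by its preset's type, or suppresses the effect if presetless.
; Spawned emitters are tracked as soft references for custom time dilation, with stale entries pruned beyond MaxEmitters.
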(event `self.ReceiveBeginPlay`
  (`self.Initialize`))

(fn `GetOverrideTemplate`
  (returns (Value :type "/Game/Assets/InfinityWeather/Footstep/Presets/BP_FootstepPreset Object Reference") (ReturnValue :type Boolean))
  (locals (CurrentVolume :type "/Game/Assets/InfinityWeather/Footstep/Blueprints/BP_FootstepVolume Object Reference") (Temp :type "/Game/Assets/InfinityWeather/Footstep/Blueprints/BP_FootstepVolume Object Reference"))
  (bind _returnvalue (`KismetArrayLibrary.Array_LastIndex` (`self.OverrideVolumes`)))
  (bind (_value _returnvalue_2) (`BlueprintMapLibrary.Map_Find` (`self.Instances`) (`.Type` (defaults `Object` (`/Game/Assets/InfinityWeather/Footstep/Blueprints/BP_FootstepVolume.Preset` (`local.CurrentVolume`))))))
  (set `local.CurrentVolume` null)
  (for _index (range (+ _returnvalue 1))
    (set `local.Temp` (`|GetArrayItem` (`self.OverrideVolumes`) (- _returnvalue _index)))
    (if (`/Game/Assets/InfinityWeather/Footstep/Blueprints/BP_FootstepVolume.IsActive` (`local.Temp`))
      (set `local.CurrentVolume` (`local.Temp`))
      (break)))
  (`/Engine/EditorBlueprintResources/StandardMacros.IsValid` (`local.CurrentVolume`)
    (:`Is Valid`
      (if (`KismetSystemLibrary.IsValidClass` (`/Game/Assets/InfinityWeather/Footstep/Blueprints/BP_FootstepVolume.Preset` (`local.CurrentVolume`)))
        (return _value _returnvalue_2)
        (else
          (return null true))))
    (:`Is Not Valid`
      (return null false))))

(fn `Initialize`
  (`BlueprintMapLibrary.Map_Clear` (`self.Instances`))
  (bind _keys (`BlueprintMapLibrary.Map_Keys` (`self.Templates`)))
  (for _array_element _keys
    (bind _returnvalue (`|GenericCreateObject` (`BlueprintMapLibrary.Map_Find` (`self.Templates`) _array_element) self))
    (`BlueprintMapLibrary.Map_Add` (`self.Instances`) _array_element _returnvalue)))

(fn `Play`
  (params (Attachement :type "/Game/Assets/InfinityWeather/Footstep/Blueprints/BS_FootstepAttachement Structure") (Intensity :type "Float (double-precision)") (Mesh :type "SkeletalMeshComponent Object Reference"))
  (locals (LFootstepInstance :type "/Game/Assets/InfinityWeather/Footstep/Presets/BP_FootstepPreset Object Reference"))
  (bind _returnvalue (`SceneComponent.GetSocketLocation` Mesh (`.Bone_2_8C52E8664CD1E2061AC7CB856D1FDA3F` (break `/Game/Assets/InfinityWeather/Footstep/Blueprints/BS_FootstepAttachement` (`local.Attachement`)))))
  ;[1 1 1] Hit detection
  (if (`self.IsActive`)
    (bind _outhit (`KismetSystemLibrary.SphereTraceSingleForObjects` (+ _returnvalue (`KismetMathLibrary.MakeVector` 0.0 0.0 (`self.FootSize`))) (- _returnvalue (`KismetMathLibrary.MakeVector` 0.0 0.0 (`self.TraceDepth`))) 10.0 (`|MakeArray` "ObjectTypeQuery1" :!type "EObjectTypeQuery Enum") false (`|MakeArray` (`self.GetOwner` Mesh)) "None" true (struct :`R` 1.0 :`A` 1.0) (struct :`G` 1.0 :`A` 1.0) 1.0))
    (`|ExecutionSequence`
      (:`then_0`
        (set `local.LFootstepInstance` null))
      (:`then_1`
        (bind (_bblockinghit _binitialoverlap _time _distance _location _impactpoint _normal _impactnormal _physmat) (`GameplayStatics.BreakHitResult` _outhit))
        (`/Engine/EditorBlueprintResources/StandardMacros.IsValid` _physmat
          (:`Is Valid`
            (set `local.LFootstepInstance` (`BlueprintMapLibrary.Map_Find` (`self.Instances`) (`KismetStringLibrary.Conv_StringToName` (`|GetEnumeratorNameAsString` (`PhysicalMaterial.SurfaceType` _physmat))))))))
      (:`then_2`
        (bind (_value _returnvalue_2) (`self.GetOverrideTemplate`))
        (if _returnvalue_2
          (set `local.LFootstepInstance` _value)))
      (:`then_3`
        ;[1 0.6384 0.4536] Final play effect
        (`/Engine/EditorBlueprintResources/StandardMacros.IsValid` (`local.LFootstepInstance`)
          (:`Is Valid`
            (bind (_spawnedaudio _spawnedemitter) (`/Game/Assets/InfinityWeather/Footstep/Presets/BP_FootstepPreset.Spawn` (`local.LFootstepInstance`) (`local.Mesh`) (`local.Attachement`) (`local.Intensity`)))
            (`/Engine/EditorBlueprintResources/StandardMacros.IsValid` _spawnedemitter
              (:`Is Valid`
                (if (not (== (`self.Dilation`) 1.0))
                  (set `ParticleSystemComponent.CustomTimeDilation` (`self.Dilation`) _spawnedemitter))
                (bind _returnvalue_3 (`KismetArrayLibrary.Array_Add` (`self.Emitters`) (`|ConvertAsset` _spawnedemitter)))
                (if (> _returnvalue_3 (`self.MaxEmitters`))
                  (`self.UpdateEmitters`))))))))))

(fn `SetCustomDilation`
  (params (Dilation :type "Float (double-precision)"))
  (set `self.Dilation` Dilation)
  (bind (_arrayindex _arrayelement) (`/Engine/EditorBlueprintResources/StandardMacros.ReverseForEachLoop` (`self.Emitters`))
    (:`LoopBody`
      (if (`KismetSystemLibrary.IsValidSoftObjectReference` _arrayelement)
        (bind _output (`|ConvertAsset` _arrayelement))
        (`/Engine/EditorBlueprintResources/StandardMacros.IsValid` _output
          (:`Is Valid`
            (if (`self.IsBeingDestroyed` _output)
              (`KismetArrayLibrary.Array_Remove` (`self.Emitters`) _arrayindex :!label _label)
              (else
                (set `ParticleSystemComponent.CustomTimeDilation` (`self.Dilation`) _output))))
          (:`Is Not Valid`
            (goto _label)))
        (else
          (goto _label))))))

(fn `SetOverrideVolume`
  (params (Volume :type "/Game/Assets/InfinityWeather/Footstep/Blueprints/BP_FootstepVolume Object Reference") (Active :type Boolean))
  (locals (InsertPosition :type Integer))
  (if Active
    (if (not (>= (`KismetArrayLibrary.Array_Find` (`self.OverrideVolumes`) (`local.Volume`)) 0))
      (set `local.InsertPosition` (`KismetArrayLibrary.Array_Length` (`self.OverrideVolumes`)))
      (for (_array_element _array_index) (`self.OverrideVolumes`)
        (if (< (`/Game/Assets/InfinityWeather/Footstep/Blueprints/BP_FootstepVolume.Priority` (`local.Volume`)) (`/Game/Assets/InfinityWeather/Footstep/Blueprints/BP_FootstepVolume.Priority` _array_element))
          (set `local.InsertPosition` _array_index)
          (break)))
      (`KismetArrayLibrary.Array_Insert` (`self.OverrideVolumes`) (`local.Volume`) (`local.InsertPosition`)))
    (else
      (`KismetArrayLibrary.Array_RemoveItem` (`self.OverrideVolumes`) (`local.Volume`)))))

(fn `UpdateEmitters`
  (bind (_arrayindex _arrayelement) (`/Engine/EditorBlueprintResources/StandardMacros.ReverseForEachLoop` (`self.Emitters`))
    (:`LoopBody`
      (if (`KismetSystemLibrary.IsValidSoftObjectReference` _arrayelement)
        (bind _output (`|ConvertAsset` _arrayelement))
        (`/Engine/EditorBlueprintResources/StandardMacros.IsValid` _output
          (:`Is Valid`
            (if (`self.IsBeingDestroyed` _output)
              (`KismetArrayLibrary.Array_Remove` (`self.Emitters`) _arrayindex :!label _label)))
          (:`Is Not Valid`
            (goto _label)))
        (else
          (goto _label))))))