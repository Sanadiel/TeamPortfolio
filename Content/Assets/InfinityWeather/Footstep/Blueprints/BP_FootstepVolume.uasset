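; Trigger volume that registers itself as a footstep override on actors carrying BP_InfinityFootstepComponent.
; Box overlap begin and end set or clear the override, and BeginPlay registers actors already inside after a zero delay.
; SetActive toggles the box and its query collision.
; IsActive reports whether the volume is enabled and its optional condition passes, comparing a named MPC_InfinityWeather scalar parameter against a required value.
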(event `self.ReceiveBeginPlay`
  (`self.SetActive` (`self.Active`))
  (`KismetSystemLibrary.Delay` 0.0)
  (if (`self.Active`)
    (for _array_element (`PrimitiveComponent.GetOverlappingActors` (`self.Box`) null)
      (bind _returnvalue (`self.GetComponentByClass` _array_element "/Game/Assets/InfinityWeather/Footstep/Blueprints/BP_InfinityFootstepComponent.BP_InfinityFootstepComponent_C"))
      (`/Engine/EditorBlueprintResources/StandardMacros.IsValid` _returnvalue
        (:`Is Valid`
          (`/Game/Assets/InfinityWeather/Footstep/Blueprints/BP_InfinityFootstepComponent.SetOverrideVolume` _returnvalue self true))))))

(event `self.Box.OnComponentBeginOverlap`
  (params (OverlappedComponent :type "PrimitiveComponent Object Reference") (OtherActor :type "Actor Object Reference") (OtherComp :type "PrimitiveComponent Object Reference") (OtherBodyIndex :type Integer) (bFromSweep :type Boolean) (SweepResult :type "HitResult Structure (by ref)"))
  (bind _returnvalue (`self.GetComponentByClass` OtherActor "/Game/Assets/InfinityWeather/Footstep/Blueprints/BP_InfinityFootstepComponent.BP_InfinityFootstepComponent_C"))
  (`/Engine/EditorBlueprintResources/StandardMacros.IsValid` _returnvalue
    (:`Is Valid`
      (`/Game/Assets/InfinityWeather/Footstep/Blueprints/BP_InfinityFootstepComponent.SetOverrideVolume` _returnvalue self true))))

(event `self.Box.OnComponentEndOverlap`
  (params (OverlappedComponent :type "PrimitiveComponent Object Reference") (OtherActor :type "Actor Object Reference") (OtherComp :type "PrimitiveComponent Object Reference") (OtherBodyIndex :type Integer))
  (bind _returnvalue (`self.GetComponentByClass` OtherActor "/Game/Assets/InfinityWeather/Footstep/Blueprints/BP_InfinityFootstepComponent.BP_InfinityFootstepComponent_C"))
  (`/Engine/EditorBlueprintResources/StandardMacros.IsValid` _returnvalue
    (:`Is Valid`
      (`/Game/Assets/InfinityWeather/Footstep/Blueprints/BP_InfinityFootstepComponent.SetOverrideVolume` _returnvalue self false))))

(fn `IsActive`
  (returns (IsActive :type Boolean))
  (bind (_requred_parameter _requred_comparsion _requred_value) (break `/Game/Assets/InfinityWeather/Footstep/Blueprints/BS_RequredParameter` (`self.Requred`)))
  (if (`self.Active`)
    (if (`|EnumEquality` _requred_parameter "NewEnumerator4")
      (return true)
      (else
        (bind _returnvalue (`KismetMaterialLibrary.GetScalarParameterValue` "/Game/Assets/InfinityWeather/Weather/Materials/MPC_InfinityWeather.MPC_InfinityWeather" (`KismetStringLibrary.Conv_StringToName` (`|GetEnumeratorNameAsString` _requred_parameter))))
        (switch `EComparisonMethod` _requred_comparsion
          (:`Equal_To`
            (return (== _requred_value _returnvalue)))
          (:`Not_Equal_To`
            (return (!= _requred_value _returnvalue)))
          (:`Greater_Than_Or_Equal_To`
            (return (>= _requred_value _returnvalue)))
          (:`Less_Than_Or_Equal_To`
            (return (<= _requred_value _returnvalue)))
          (:`Greater_Than`
            (return (> _returnvalue _requred_value)))
          (:`Less_Than`
            (return (< _requred_value _returnvalue))))))
    (else
      (return false))))

(fn `SetActive`
  (params (Activate :type Boolean))
  (bind _output_get (set `self.Active` Activate))
  (`ActorComponent.SetActive` (`self.Box`) _output_get false)
  (if (`self.Active`)
    (`PrimitiveComponent.SetCollisionEnabled` (`self.Box`) "QueryOnly")
    (else
      (`PrimitiveComponent.SetCollisionEnabled` (`self.Box`) "NoCollision"))))

(fn `UserConstructionScript`
  (`self.SetActive` (`self.Active`)))