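; BP_InfinityFog is a spherical local fog volume that supplies weighted atmosphere influence to the Infinity Weather system.
; The construction script scales the sphere and mesh to the shape radius, drives a dynamic material's color and density, and refreshes any assigned controller's atmosphere.
; At BeginPlay it finds a controller if needed and registers in its FogVolumes.
; GetSampleWeight returns a radial falloff weight for a location, zero when inactive or outside.
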(event `self.ReceiveBeginPlay`
  (`/Engine/EditorBlueprintResources/StandardMacros.IsValid` (`self.Controller`)
    (:`Is Valid`
      (`self.SetController` (`self.Controller`)))
    (:`Is Not Valid`
      (bind _returnvalue (`GameplayStatics.GetActorOfClass` "/Game/Assets/InfinityWeather/BP_InfinityWeatherController.BP_InfinityWeatherController_C"))
      (`self.SetController` _returnvalue))))

(fn `GetSampleWeight`
  (params (Location :type "Vector Structure"))
  (returns (Weight :type "Float (double-precision)"))
  (locals (Distance :type "Float (double-precision)" :default 0.0))
  (if (`self.Active`)
    (set `local.Distance` (`KismetMathLibrary.VSize` (`KismetMathLibrary.InverseTransformLocation` (`KismetMathLibrary.MakeTransform` (`self.K2_GetActorLocation`) (`self.K2_GetActorRotation`) (`self.ShapeRadius`)) (`local.Location`))))
    (if (< (`local.Distance`) 1.0)
      (return (`KismetMathLibrary.MultiplyMultiply_FloatFloat` (`KismetMathLibrary.MapRangeClamped` (`local.Distance`) 1.0 (- 1.0 (`KismetMathLibrary.FMax` (`self.AtmosphereFalloff`) 0.01)) 0.0 (`.Weight_16_E2EDC8D24F399AC13C51FAA90BC6C5FB` (break `/Game/Assets/InfinityWeather/Environment/Fog/BS_InfinityAtmosphere` (`self.Atmosphere`)))) (`self.AtmosphereFalloffExp`)))
      (else
        (return 0.0)))
    (else
      (return 0.0))))

(fn `GetShape`
  (returns (NewParam :type "LinearColor Structure") (Radius :type "Vector Structure"))
  (return (`KismetMathLibrary.Conv_VectorToLinearColor` (`self.K2_GetActorLocation`)) (`self.ShapeRadius`)))

(fn `SetController`
  (params (Controller :type "/Game/Assets/InfinityWeather/BP_InfinityWeatherController Object Reference"))
  (`/Engine/EditorBlueprintResources/StandardMacros.IsValid` Controller
    (:`Is Valid`
      (bind _output_get (set `self.Controller` Controller))
      (`KismetArrayLibrary.Array_AddUnique` (`/Game/Assets/InfinityWeather/BP_InfinityWeatherController.FogVolumes` _output_get) self))))

(fn `UserConstructionScript`
  (bind _controller (`self.Controller`))
  (bind _shapedensity (`self.ShapeDensity`))
  (bind _returnvalue (/ (`self.ShapeRadius`) 50.0))
  (`|ExecutionSequence`
    (:`then_0`
      (`SphereComponent.SetSphereRadius` (`self.Sphere`) 50.0 true)
      (`SceneComponent.SetWorldScale3D` (`self.Sphere`) _returnvalue)
      (`SceneComponent.SetWorldScale3D` (`self.Mesh`) _returnvalue)
      (bind _returnvalue_2 (`PrimitiveComponent.CreateDynamicMaterialInstance` (`self.Mesh`) 0 null "None"))
      (set `self.SphereMaterial` _returnvalue_2)
      (`MaterialInstanceDynamic.SetVectorParameterValue` (`self.SphereMaterial`) "AtmosphereColor" (`self.ShapeColor`))
      (`MaterialInstanceDynamic.SetScalarParameterValue` (`self.SphereMaterial`) "AtmosphereDensity" _shapedensity)
      (`SceneComponent.SetVisibility` (`self.Mesh`) (and (> _shapedensity 0.0) (`self.Active`)) false))
    (:`then_1`
      (bind _outactors (`GameplayStatics.GetAllActorsOfClass` "/Game/Assets/InfinityWeather/BP_InfinityWeatherController.BP_InfinityWeatherController_C"))
      (for _ _outactors
        _))
    (:`then_2`
      (`/Engine/EditorBlueprintResources/StandardMacros.IsValid` _controller
        (:`Is Valid`
          (`/Game/Assets/InfinityWeather/BP_InfinityWeatherController.UpdateAtmosphere` _controller 0.0))))))