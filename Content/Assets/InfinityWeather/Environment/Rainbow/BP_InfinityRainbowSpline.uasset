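; Spline-driven rainbow actor that builds a mesh along its spline at construction.
; CreateMesh adds a shadowless spline mesh per segment, each with a dynamic material given segment index, scaled length and colors.
; UpdateSplineMesh fits tangents, scale and roll around the segment's midpoint up vector.
; Optional FixSpline derives point up vectors from consecutive tangent cross products, sign-matched to avoid flips.
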(fn `CreateMesh`
  (locals (DynamicMaterial :type "MaterialInstanceDynamic Object Reference") (StartIndex :type Integer) (EndIndex :type Integer) (SplineMesh :type "SplineMeshComponent Object Reference") (StartDistance :type "Float (double-precision)") (EndDistance :type "Float (double-precision)") (MiddleDistance :type "Float (double-precision)"))
  (bind _splinemeshes (`self.SplineMeshes`))
  ;[1 1 1] Create simple tube spline mesh
  (for _array_element _splinemeshes
    (`ActorComponent.K2_DestroyComponent` _array_element))
  (`KismetArrayLibrary.Array_Clear` _splinemeshes)
  (if (`self.FixSplineDirection`)
    (`self.FixSpline`))
  (for _index (range (+ (- (`SplineComponent.GetNumberOfSplinePoints` (`self.Spline`)) 2) 1))
    (set `local.StartIndex` _index)
    (set `local.EndIndex` (+ _index 1))
    (bind _returnvalue (`AddComponent|NODE_AddSplineMeshComponent-0`))
    (bind _output_get (set `local.SplineMesh` _returnvalue))
    (`KismetArrayLibrary.Array_Add` (`self.SplineMeshes`) _output_get)
    (`StaticMeshComponent.SetStaticMesh` _output_get (`self.StaticMesh`))
    (`SplineMeshComponent.SetForwardAxis` (`local.SplineMesh`) (`self.ForwardAxis`) true)
    (`SceneComponent.K2_AttachToComponent` (`local.SplineMesh`) (`self.Spline`) "None" "KeepRelative" "KeepRelative" "KeepRelative" true)
    (`PrimitiveComponent.SetCastShadow` (`local.SplineMesh`) false)
    (`PrimitiveComponent.SetTranslucentSortPriority` (`local.SplineMesh`) (`self.TranslucencySortPriority`))
    (`self.UpdateSplineMesh` (`local.StartIndex`))
    ;[1 1 1] Material
    (bind _returnvalue_2 (`PrimitiveComponent.CreateDynamicMaterialInstance` (`local.SplineMesh`) 0 (`self.Material`) "None"))
    (`KismetArrayLibrary.Array_Add` (`self.MaterialInstances`) _returnvalue_2)
    (set `local.DynamicMaterial` _returnvalue_2)
    (`MaterialInstanceDynamic.SetScalarParameterValue` (`local.DynamicMaterial`) "BeamUVIndex" (`KismetMathLibrary.Conv_IntToDouble` (`local.StartIndex`)))
    (`MaterialInstanceDynamic.SetScalarParameterValue` (`local.DynamicMaterial`) "BeamUVLength" (* (`KismetMathLibrary.Conv_IntToDouble` (- (`SplineComponent.GetNumberOfSplinePoints` (`self.Spline`)) 1)) (`self.TextureScale`)))
    (`MaterialInstanceDynamic.SetVectorParameterValue` (`local.DynamicMaterial`) "GlowColor" (`self.GlowColor`))
    (`MaterialInstanceDynamic.SetVectorParameterValue` (`local.DynamicMaterial`) "LineColor" (`self.LineColor`))))

(fn `FixSpline`
  (locals (PrevDirection :type "Vector Structure"))
  (bind _spline (`self.Spline`))
  (set `local.PrevDirection` (`SplineComponent.GetUpVectorAtSplinePoint` (`self.Spline`) 0 "World"))
  (for _index (range 1 (`SplineComponent.GetNumberOfSplinePoints` (`self.Spline`)))
    (bind _returnvalue (`KismetMathLibrary.Cross_VectorVector` (`SplineComponent.GetTangentAtSplinePoint` _spline _index "World") (`SplineComponent.GetTangentAtSplinePoint` _spline (- _index 1) "World")))
    (bind _returnvalue_2 (select `bool` (> (`KismetMathLibrary.Dot_VectorVector` _returnvalue (`local.PrevDirection`)) 0.0) :`false` (* _returnvalue -1.0) :`true` _returnvalue))
    (`SplineComponent.SetUpVectorAtSplinePoint` (`self.Spline`) _index _returnvalue_2 "World" true)
    (set `local.PrevDirection` _returnvalue_2)))

(fn `UpdateSplineMesh`
  (params (Index :type Integer))
  (locals (StartDistance :type "Float (double-precision)") (EndDistance :type "Float (double-precision)") (MiddleDistance :type "Float (double-precision)") (StartIndex :type Integer) (EndIndex :type Integer) (SplineMesh :type "SplineMeshComponent Object Reference"))
  (bind _spline (`self.Spline`))
  (bind _startindex (`local.StartIndex`))
  (bind _endindex (`local.EndIndex`))
  (bind _spline_2 (`self.Spline`))
  (bind (_returnvalue_x _returnvalue_y _returnvalue_z) (`KismetMathLibrary.BreakVector` (* (`SplineComponent.GetScaleAtDistanceAlongSpline` (`self.Spline`) (`local.StartDistance`)) (`self.WidthScale`))))
  (bind (_returnvalue_x_2 _returnvalue_y_2 _returnvalue_z_2) (`KismetMathLibrary.BreakVector` (* (`SplineComponent.GetScaleAtDistanceAlongSpline` (`self.Spline`) (`local.EndDistance`)) (`self.WidthScale`))))
  (bind _returnvalue (`KismetMathLibrary.Lerp` (`SplineComponent.GetDistanceAlongSplineAtSplinePoint` (`self.Spline`) (`local.StartIndex`)) (`SplineComponent.GetDistanceAlongSplineAtSplinePoint` (`self.Spline`) (`local.EndIndex`)) 0.5))
  (bind _returnvalue_2 (`KismetMathLibrary.NegateRotator` (`SplineComponent.GetRotationAtDistanceAlongSpline` (`self.Spline`) _returnvalue "Local")))
  (bind _returnvalue_roll (`KismetMathLibrary.BreakRotator` (`KismetMathLibrary.ComposeRotators` (`SplineComponent.GetRotationAtSplinePoint` (`self.Spline`) (`local.EndIndex`) "Local") _returnvalue_2)))
  (bind _returnvalue_roll_2 (`KismetMathLibrary.BreakRotator` (`KismetMathLibrary.ComposeRotators` (`SplineComponent.GetRotationAtSplinePoint` (`self.Spline`) (`local.StartIndex`) "Local") _returnvalue_2)))
  ;[1 1 1] Init basic info
  (set `local.SplineMesh` (`|GetArrayItem` (`self.SplineMeshes`) Index))
  (bind _output_get (set `local.StartIndex` Index))
  (set `local.EndIndex` (+ _output_get 1))
  (set `local.StartDistance` (`SplineComponent.GetDistanceAlongSplineAtSplinePoint` (`self.Spline`) (`local.StartIndex`)))
  (set `local.EndDistance` (`SplineComponent.GetDistanceAlongSplineAtSplinePoint` (`self.Spline`) (`local.EndIndex`)))
  (set `local.MiddleDistance` (`KismetMathLibrary.Lerp` (`local.StartDistance`) (`local.EndDistance`) 0.5))
  ;[1 1 1] Start and End location
  (`SplineMeshComponent.SetStartAndEnd` (`local.SplineMesh`) (`SplineComponent.GetLocationAtSplinePoint` _spline_2 _startindex "Local") (`SplineComponent.GetTangentAtSplinePoint` _spline_2 _startindex "Local") (`SplineComponent.GetLocationAtSplinePoint` _spline _endindex "Local") (`SplineComponent.GetTangentAtSplinePoint` _spline _endindex "Local") false)
  ;[1 1 1] Start end scale
  (`SplineMeshComponent.SetStartScale` (`local.SplineMesh`) (`KismetMathLibrary.MakeVector2D` _returnvalue_y _returnvalue_z) false)
  (`SplineMeshComponent.SetEndScale` (`local.SplineMesh`) (`KismetMathLibrary.MakeVector2D` _returnvalue_y_2 _returnvalue_z_2) false)
  ;[1 1 1] Up direction
  (`SplineMeshComponent.SetSplineUpDir` (`local.SplineMesh`) (`SplineComponent.GetUpVectorAtDistanceAlongSpline` (`self.Spline`) _returnvalue "Local") false)
  ;[1 1 1] Roll
  (`SplineMeshComponent.SetStartRoll` (`local.SplineMesh`) (`KismetMathLibrary.DegreesToRadians` _returnvalue_roll_2) false)
  (`SplineMeshComponent.SetEndRoll` (`local.SplineMesh`) (`KismetMathLibrary.DegreesToRadians` _returnvalue_roll) true))

(fn `UserConstructionScript`
  (`KismetArrayLibrary.Array_Clear` (`self.SplineMeshes`))
  (`KismetArrayLibrary.Array_Clear` (`self.MaterialInstances`))
  (`self.CreateMesh`))