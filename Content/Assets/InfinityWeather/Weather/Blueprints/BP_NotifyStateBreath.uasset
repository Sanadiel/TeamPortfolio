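; BP_NotifyStateBreath is an animation notify state that toggles a character's breath effect in the InfinityWeather system during an animation window.
; Notify begin enables breath and notify end disables it, both through a shared SetBreath function.
; SetBreath finds the BP_InfinityPawnComponent on the mesh's owner and, if valid, calls SetOwnerBreath with the state and mesh.
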(fn `Received_NotifyBegin`
  (params (MeshComp :type "SkeletalMeshComponent Object Reference") (Animation :type "AnimSequenceBase Object Reference") (TotalDuration :type "Float (double-precision)"))
  (returns (ReturnValue :type Boolean))
  (`self.SetBreath` MeshComp true)
  (return false))

(fn `Received_NotifyEnd`
  (params (MeshComp :type "SkeletalMeshComponent Object Reference") (Animation :type "AnimSequenceBase Object Reference"))
  (returns (ReturnValue :type Boolean))
  (`self.SetBreath` MeshComp)
  (return false))

(fn `SetBreath`
  (params (Mesh :type "SkeletalMeshComponent Object Reference") (Enable :type Boolean))
  (bind _returnvalue (`Actor.GetComponentByClass` (`ActorComponent.GetOwner` Mesh) "/Game/Assets/InfinityWeather/Weather/Blueprints/BP_InfinityPawnComponent.BP_InfinityPawnComponent_C"))
  (`/Engine/EditorBlueprintResources/StandardMacros.IsValid` _returnvalue
    (:`Is Valid`
      (`/Game/Assets/InfinityWeather/Weather/Blueprints/BP_InfinityPawnComponent.SetOwnerBreath` _returnvalue (`local.Enable`) (`local.Mesh`)))))