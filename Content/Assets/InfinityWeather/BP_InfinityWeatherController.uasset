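; World weather controller actor that drives global wind, precipitation, ground wetness and snow, and atmosphere.
; Setters start timed blends, advanced by a looping timer, while Tick accumulates wind offsets.
; Results feed MPC_InfinityWeather for materials, height fog blended with fog volumes at the camera, wind-affected emitters, and precipitation spawned as child actors that are removed after fading out.
; Location queries expose wind, precipitation and fog data, plus a sphere-trace wind occlusion test.
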(event `self.ReceiveBeginPlay`
  ;[1 1 1] Initialization of all effects
  (set `self.PreviewFogActor` null)
  (`self.UpdateAccumulation` -1.0)
  (`self.UpdateAtmosphere` -1.0)
  (set `self.WindDistance` 0.0)
  (`self.UpdateWindDirection` -1.0)
  (`KismetSystemLibrary.K2_SetTimerDelegate` (delegate `UpdateWorld`) (`self.UpdateWorldFrequency`) true))

(event `UpdateWorld`
  (`self.UpdateWindDirection` (`self.UpdateWorldFrequency`))
  (`self.UpdateAccumulation` (`self.UpdateWorldFrequency`))
  (`self.UpdateAtmosphere` (`self.UpdateWorldFrequency`)))

(event `self.ReceiveTick`
  (params (DeltaSeconds :type "Float (single-precision)"))
  ;[1 1 1] Update wind offsets for clouds and wind based effects
  (`self.UpdateWindOffset` DeltaSeconds))

(event `BindDestroyEffect`
  (params (Actor :type "/Game/Assets/InfinityWeather/Precipitation/Base/BP_InfinityPrecipitation Object Reference"))
  ;[1 1 1] Removing pericpitation when tis finished
  (add `/Game/Assets/InfinityWeather/Precipitation/Base/BP_InfinityPrecipitation.OnParticlCountBlendFinished` Actor (delegate `DestroyPrecipitation`)))

(event `DestroyPrecipitation`
  (params (Effect :type "/Game/Assets/InfinityWeather/Precipitation/Base/BP_InfinityPrecipitation Object Reference") (Remove :type Boolean))
  ;[1 1 1] Removing pericpitation when tis finished
  (if Remove
    (`KismetArrayLibrary.Array_RemoveItem` (`self.PrecipitationActors`) Effect)
    (bind (_arrayindex _arrayelement) (`/Engine/EditorBlueprintResources/StandardMacros.ReverseForEachLoop` (`self.PrecipitationComponents`))
      (:`LoopBody`
        (if (== (`ChildActorComponent.ChildActor` _arrayelement) Effect)
          (`ActorComponent.K2_DestroyComponent` _arrayelement)
          (`KismetArrayLibrary.Array_Remove` (`self.PrecipitationComponents`) _arrayindex))))))

(fn `AddPostProcessComponent`
  (params (Component :type "/Game/Assets/InfinityWeather/PostProcess/Blueprints/BP_InfinityWeatherComponent Object Reference (by ref)"))
  (`KismetArrayLibrary.Array_AddUnique` (`self.PostProcessComponents`) Component))

(fn `GetFogDataAtLocation`
  (params (Location :type "Vector Structure"))
  (returns (Data :type "/Game/Assets/InfinityWeather/Environment/Fog/BS_InfinityAtmosphere Structure"))
  (locals (Weight :type "Float (double-precision)") (ScaledWeight :type "Float (double-precision)") (SumWeights :type "Float (double-precision)") (Temp :type "/Game/Assets/InfinityWeather/Environment/Fog/BS_InfinityAtmosphere Structure"))
  (bind (_temp_weight _temp_fogdensity _temp_fogheightfalloff _temp_fogcolor _temp_distortion _temp_humidity _temp_temperature) (break `/Game/Assets/InfinityWeather/Environment/Fog/BS_InfinityAtmosphere` (`local.Temp`)))
  (bind _weight (`local.Weight`))
  (bind (_temp_weight_2 _temp_fogdensity_2 _temp_fogheightfalloff_2 _temp_fogcolor_2 _temp_distortion_2 _temp_humidity_2 _temp_temperature_2) (break `/Game/Assets/InfinityWeather/Environment/Fog/BS_InfinityAtmosphere` (`local.Temp`)))
  (`|ExecutionSequence`
    (:`then_0`
      (if (> (`KismetArrayLibrary.Array_Length` (`self.FogVolumes`)) 0)
        (set `local.Temp` (`self.AtmosphereSettings`))
        (set `local.SumWeights` 1.0)
        (for _array_element (`self.FogVolumes`)
          (`/Engine/EditorBlueprintResources/StandardMacros.IsValid` _array_element
            (:`Is Valid`
              (bind _weight_2 (`/Game/Assets/InfinityWeather/Environment/Fog/BP_InfinityFog.GetSampleWeight` _array_element (`local.Location`)))
              (if (> _weight_2 0.0)
                (bind _output_get (set `local.ScaledWeight` (/ _weight_2 (`.Weight_16_E2EDC8D24F399AC13C51FAA90BC6C5FB` (break `/Game/Assets/InfinityWeather/Environment/Fog/BS_InfinityAtmosphere` (`self.AtmosphereSettings`))))))
                (bind (_atmosphere_weight _atmosphere_fogdensity _atmosphere_fogheightfalloff _atmosphere_fogcolor _atmosphere_distortion _atmosphere_humidity _atmosphere_temperature) (break `/Game/Assets/InfinityWeather/Environment/Fog/BS_InfinityAtmosphere` (`/Game/Assets/InfinityWeather/Environment/Fog/BP_InfinityFog.Atmosphere` _array_element)))
                (set `local.Temp` (make `/Game/Assets/InfinityWeather/Environment/Fog/BS_InfinityAtmosphere` 1.0 (+ _temp_fogdensity (* _output_get _atmosphere_fogdensity)) (+ _temp_fogheightfalloff (* _output_get _atmosphere_fogheightfalloff)) (+ _temp_fogcolor (* _atmosphere_fogcolor _output_get)) (+ _temp_distortion (* _output_get _atmosphere_distortion)) (+ _temp_humidity (* _output_get _atmosphere_humidity)) (+ _temp_temperature (* _output_get _atmosphere_temperature))))
                (set `local.SumWeights` (+ (`local.SumWeights`) (`local.ScaledWeight`)))))))
        (if (`KismetMathLibrary.NearlyEqual_FloatFloat` (`local.SumWeights`) 1.0)
          (return (`self.AtmosphereSettings`))
          (else
            (set `local.Weight` (/ 1.0 (`local.SumWeights`)))
            (return (make `/Game/Assets/InfinityWeather/Environment/Fog/BS_InfinityAtmosphere` 1.0 (* _weight _temp_fogdensity_2) (* _weight _temp_fogheightfalloff_2) (* _temp_fogcolor_2 _weight) (* _weight _temp_distortion_2) (* _weight _temp_humidity_2) (* _weight _temp_temperature_2)))))))
    (:`then_1`
      (return (`self.AtmosphereSettings`)))))

(fn `GetPrecipitationDataAtLocation`
  (params (Location :type "Vector Structure"))
  (returns (Rain :type "Float (double-precision)") (Snow :type "Float (double-precision)") (Wind :type "Float (double-precision)") (Force :type "Vector Structure"))
  (locals (ResultRain :type "Float (double-precision)" :default 0.0) (ResultSnow :type "Float (double-precision)" :default 0.0) (ResultWind :type "Float (double-precision)" :default 0.0) (ResultForce :type "Vector Structure"))
  (set `local.ResultRain` 0.0)
  (set `local.ResultSnow` 0.0)
  (set `local.ResultWind` 0.0)
  (set `local.ResultForce` (0.0 0.0 0.0))
  (for _array_element (`self.PrecipitationActors`)
    (bind (_rain _snow _wind _force) (`/Game/Assets/InfinityWeather/Precipitation/Base/BP_InfinityPrecipitation.GetPrecipitationAtPoint` _array_element (`local.Location`)))
    (set `local.ResultRain` (+ _rain (`local.ResultRain`)))
    (set `local.ResultSnow` (+ _snow (`local.ResultSnow`)))
    (set `local.ResultWind` (+ _wind (`local.ResultWind`)))
    (set `local.ResultForce` (+ _force (`local.ResultForce`))))
  (return (`local.ResultRain`) (`local.ResultSnow`) (`local.ResultWind`) (`KismetMathLibrary.Normal` (`local.ResultForce`))))

(fn `GetRandomWindForce`
  (params (LengthRange :type "Vector2D Structure" :default (0.0 1.0)))
  (returns (Force :type "Vector Structure"))
  (return (* (`KismetMathLibrary.Normal` (* (`KismetMathLibrary.RandomUnitVector`) (1.0 1.0 0.0))) (`KismetMathLibrary.RandomFloatInRange` LengthRange_X LengthRange_Y))))

(fn `GetWindDataAtLocation`
  (params (Location :type "Vector Structure"))
  (returns (Force :type "Vector Structure") (Damage :type "Float (double-precision)"))
  (return (`self.WindForce`) (`self.WindDamage`)))

(fn `IsWindOccludedActor`
  (params (Actor :type "Actor Object Reference") (TestDistance :type "Float (double-precision)"))
  (returns (ReturnValue :type Boolean))
  (locals (ActorLocation :type "Vector Structure" :default (0.0 0.0 0.0)) (TraceForce :type "Vector Structure"))
  (bind _output_get (set `local.ActorLocation` (`self.K2_GetActorLocation` Actor)))
  (bind (_rain _snow _wind _force) (`self.GetPrecipitationDataAtLocation` _output_get))
  (bind (_outhit _returnvalue) (`KismetSystemLibrary.SphereTraceSingle` (`local.ActorLocation`) (- (`local.ActorLocation`) (* (`KismetMathLibrary.Normal` _force) TestDistance)) 20.0 "TraceTypeQuery2" false (`|MakeArray` (`local.Actor`))))
  (return _returnvalue))

(fn `SetAccumulation`
  (params (BlendDuration :type "Float (double-precision)" :default 10.0) (WetSurface :type "Float (double-precision)") (WetDisplacement :type "Float (double-precision)") (SnowySurface :type "Float (double-precision)") (SnowyDisplacement :type "Float (double-precision)") (DisplacementAccumulation :type "Float (double-precision)" :default 1.0))
  (set `self.GroundTo` (make `LinearColor` WetSurface WetDisplacement SnowySurface SnowyDisplacement))
  (set `self.DisplacementAccumulation` DisplacementAccumulation)
  (if (> (`local.BlendDuration`) 0.0)
    (set `self.GroundBlendSpeed` (/ 1.0 (`local.BlendDuration`)))
    (set `self.GroundBlendTime` 0.0)
    (set `self.GroundFrom` (make `LinearColor` (`self.WetSurface`) (`self.WetDisplacement`) (`self.SnowySurface`) (`self.SnowyDisplacement`)))
    (else
      (set `self.GroundBlendSpeed` 10000.0)
      (set `self.GroundBlendTime` 1.0)
      (set `self.GroundFrom` (`self.GroundTo`))
      (set `self.WetSurface` WetSurface)
      (set `self.WetDisplacement` WetDisplacement)
      (set `self.SnowySurface` SnowySurface)
      (set `self.SnowyDisplacement` SnowyDisplacement)
      (`self.UpdateAccumulation` -1.0))))

(fn `SetAtmosphere`
  (params (BlendDuration :type "Float (double-precision)" :default 10.0) (Data :type "/Game/Assets/InfinityWeather/Environment/Fog/BS_InfinityAtmosphere Structure"))
  (bind _blendduration (`local.BlendDuration`))
  (set `self.GlobalFogAirTo` Data)
  (if (> _blendduration 0.0)
    (set `self.AirBlendSpeed` (/ 1.0 _blendduration))
    (set `self.AirBlendTime` 0.0)
    (set `self.GlobalFogAirFrom` (`self.AtmosphereSettings`))
    (else
      (set `self.AirBlendSpeed` 0.0)
      (set `self.AirBlendTime` 1.0)
      (set `self.AtmosphereSettings` (`self.GlobalFogAirTo`))
      (`self.UpdateAtmosphere` -1.0))))

(fn `SetDefault`
  (`self.SetWind` -1.0 (`self.WindForce`) (`self.WindDamage`))
  (`self.SetPrecipitation` -1.0 (`self.PrecipitationEffectClass`) (`self.PrecipitationCount`))
  (`self.SetAccumulation` -1.0 (`self.WetSurface`) (`self.WetDisplacement`) (`self.SnowySurface`) (`self.SnowyDisplacement`) (`self.DisplacementAccumulation`))
  (`self.SetAtmosphere` -1.0 (`self.AtmosphereSettings`))
  (`GameplayStatics.GetAllActorsOfClass` null))

(fn `SetPrecipitation`
  (params (BlendDuration :type "Float (double-precision)" :default 10.0) (EffectClass :type "/Game/Assets/InfinityWeather/Precipitation/Base/BP_InfinityPrecipitation Class Reference") (ParticleCount :type Integer :default 5000) (Animation :type "CurveFloat Object Reference") (Override :type Boolean :default true))
  (returns (Handle :type "/Game/Assets/InfinityWeather/Precipitation/Base/BP_InfinityPrecipitation Object Reference"))
  (locals (ChildActor :type "ChildActorComponent Object Reference") (TempEffect :type "/Game/Assets/InfinityWeather/Precipitation/Base/BP_InfinityPrecipitation Object Reference"))
  (`|ExecutionSequence`
    (:`then_0`
      (if (`local.Override`)
        (for _array_element (`self.PrecipitationComponents`)
          (`/Engine/EditorBlueprintResources/StandardMacros.IsValid` _array_element
            (:`Is Valid`
              (bind _asbp_infinity_precipitation (cast `/Game/Assets/InfinityWeather/Precipitation/Base/BP_InfinityPrecipitation` (`ChildActorComponent.ChildActor` _array_element)))
              (`/Game/Assets/InfinityWeather/Precipitation/Base/BP_InfinityPrecipitation.SetParticeCountBlend` _asbp_infinity_precipitation 0 (`local.BlendDuration`) (`local.Animation`) true))))))
    (:`then_1`
      (if (`KismetSystemLibrary.IsValidClass` (`local.EffectClass`))
        (`|ExecutionSequence`
          (:`then_0`
            (bind _returnvalue (`AddComponent|NODE_AddChildActorComponent-2`))
            (set `local.ChildActor` _returnvalue)
            (`ChildActorComponent.SetChildActorClass` (`local.ChildActor`) (`local.EffectClass`))
            (`KismetArrayLibrary.Array_Add` (`self.PrecipitationComponents`) (`local.ChildActor`))
            (bind _asbp_infinity_precipitation_2 (cast `/Game/Assets/InfinityWeather/Precipitation/Base/BP_InfinityPrecipitation` (`ChildActorComponent.ChildActor` (`local.ChildActor`))))
            (set `local.TempEffect` _asbp_infinity_precipitation_2)
            (`/Game/Assets/InfinityWeather/Precipitation/Base/BP_InfinityPrecipitation.SetVolumeSize` (`local.TempEffect`) (100000.0 100000.0 100000.0) true)
            (`self.BindDestroyEffect` (`local.TempEffect`)))
          (:`then_1`
            (if (<= (`local.BlendDuration`) 0.0)
              (`/Game/Assets/InfinityWeather/Precipitation/Base/BP_InfinityPrecipitation.SetParticleCount` (`local.TempEffect`) (`local.ParticleCount`))
              (else
                (`/Game/Assets/InfinityWeather/Precipitation/Base/BP_InfinityPrecipitation.SetParticleCount` (`local.TempEffect`) 0)
                (`/Game/Assets/InfinityWeather/Precipitation/Base/BP_InfinityPrecipitation.SetParticeCountBlend` (`local.TempEffect`) (`local.ParticleCount`) (`local.BlendDuration`) (`local.Animation`) false))))
          (:`then_2`
            (`/Game/Assets/InfinityWeather/Precipitation/Base/BP_InfinityPrecipitation.SetWindForce` (`local.TempEffect`) 0.0 (`self.WindForceTo`))))
        (else
          (set `local.TempEffect` null))))
    (:`then_2`
      (return (`local.TempEffect`)))))

(fn `SetWind`
  (params (BlendDuration :type "Float (double-precision)" :default 10.0) (Force :type "Vector Structure") (Damage :type "Float (double-precision)"))
  (set `self.WindForceTo` Force)
  (set `self.WindDamageTo` (`local.Damage`))
  (`self.UpdateWindAffectedActors` (`local.BlendDuration`))
  (if (> (`local.BlendDuration`) 0.0)
    (set `self.WindBlendSpeed` (/ 1.0 (`local.BlendDuration`)))
    (set `self.WindBlendTime` 0.0)
    (set `self.WindDamageFrom` (`self.WindDamage`))
    (set `self.WindForceFrom` (`self.WindForce`))
    (else
      (set `self.WindBlendSpeed` 0.0)
      (set `self.WindForce` (`self.WindForceTo`))
      (set `self.WindDamage` (`self.WindDamageTo`))
      (set `self.WindBlendTime` 1.0)
      (`self.UpdateWindDirection` -1.0))))

(fn `UpdateAccumulation`
  (params (DeltaTime :type "Float (double-precision)"))
  (locals (GroundParams :type "LinearColor Structure") (DisplaceParams :type "LinearColor Structure"))
  (bind (_groundparams_r _groundparams_g _groundparams_b _groundparams_a) (break `LinearColor` (`local.GroundParams`)))
  ;[1 1 1] Update materials
  (if (< (`self.GroundBlendTime`) 1.0)
    (set `self.GroundBlendTime` (`KismetMathLibrary.FMin` (+ (`self.GroundBlendTime`) (* DeltaTime (`self.GroundBlendSpeed`))) 1.0))
    ;[1 1 1] Apply parameters
    (set `local.GroundParams` (`KismetMathLibrary.LinearColorLerp` (`self.GroundFrom`) (`self.GroundTo`) (`self.GroundBlendTime`)) :!label _label)
    (set `self.WetSurface` _groundparams_r)
    (set `self.WetDisplacement` _groundparams_g)
    (set `self.SnowySurface` _groundparams_b)
    (set `self.SnowyDisplacement` _groundparams_a)
    (`KismetMaterialLibrary.SetScalarParameterValue` "/Game/Assets/InfinityWeather/MPC_InfinityWeather.MPC_InfinityWeather" "SurfaceSnowy" (`self.SnowySurface`))
    (`KismetMaterialLibrary.SetScalarParameterValue` "/Game/Assets/InfinityWeather/MPC_InfinityWeather.MPC_InfinityWeather" "SurfaceWet" (`self.WetSurface`))
    (`KismetMaterialLibrary.SetScalarParameterValue` "/Game/Assets/InfinityWeather/MPC_InfinityWeather.MPC_InfinityWeather" "DisplacementSnowy" (`self.SnowyDisplacement`))
    (`KismetMaterialLibrary.SetScalarParameterValue` "/Game/Assets/InfinityWeather/MPC_InfinityWeather.MPC_InfinityWeather" "DisplacementWet" (`self.WetDisplacement`))
    (elif (< (`local.DeltaTime`) 0.0)
      (goto _label))))

(fn `UpdateAtmosphere`
  (params (DeltaTime :type "Float (double-precision)"))
  (bind _returnvalue (`GameplayStatics.GetPlayerCameraManager` 0))
  (bind (_finalfogair_weight _finalfogair_fogdensity _finalfogair_fogheightfalloff _finalfogair_fogcolor) (break `/Game/Assets/InfinityWeather/Environment/Fog/BS_InfinityAtmosphere` (`self.FinalFogAir`)))
  (bind _previewfogactor (`self.PreviewFogActor`))
  (bind (_globalfogairfrom_weight _globalfogairfrom_fogdensity _globalfogairfrom_fogheightfalloff _globalfogairfrom_fogcolor _globalfogairfrom_distortion _globalfogairfrom_humidity _globalfogairfrom_temperature) (break `/Game/Assets/InfinityWeather/Environment/Fog/BS_InfinityAtmosphere` (`self.GlobalFogAirFrom`)))
  (bind (_globalfogairto_weight _globalfogairto_fogdensity _globalfogairto_fogheightfalloff _globalfogairto_fogcolor _globalfogairto_distortion _globalfogairto_humidity _globalfogairto_temperature) (break `/Game/Assets/InfinityWeather/Environment/Fog/BS_InfinityAtmosphere` (`self.GlobalFogAirTo`)))
  (bind _component (`ExponentialHeightFog.Component` (`self.ExponentialHeightFog`)))
  (`|ExecutionSequence`
    (:`then_0`
      (if (< (`self.AirBlendTime`) 1.0)
        (set `self.AirBlendTime` (`KismetMathLibrary.FMin` (+ (`self.AirBlendTime`) (* (`local.DeltaTime`) (`self.AirBlendSpeed`))) 1.0))
        (set `self.AtmosphereSettings` (make `/Game/Assets/InfinityWeather/Environment/Fog/BS_InfinityAtmosphere` (`KismetMathLibrary.Lerp` _globalfogairfrom_weight _globalfogairto_weight (`self.AirBlendTime`)) (`KismetMathLibrary.Lerp` _globalfogairfrom_fogdensity _globalfogairto_fogdensity (`self.AirBlendTime`)) (`KismetMathLibrary.Lerp` _globalfogairfrom_fogheightfalloff _globalfogairto_fogheightfalloff (`self.AirBlendTime`)) (`KismetMathLibrary.LinearColorLerp` _globalfogairfrom_fogcolor _globalfogairto_fogcolor (`self.AirBlendTime`)) (`KismetMathLibrary.Lerp` _globalfogairfrom_distortion _globalfogairto_distortion (`self.AirBlendTime`)) (`KismetMathLibrary.Lerp` _globalfogairfrom_humidity _globalfogairto_humidity (`self.AirBlendTime`)) (`KismetMathLibrary.Lerp` _globalfogairfrom_temperature _globalfogairto_temperature (`self.AirBlendTime`))))))
    (:`then_1`
      (`/Engine/EditorBlueprintResources/StandardMacros.IsValid` _returnvalue
        (:`Is Valid`
          (bind _data (`self.GetFogDataAtLocation` (`self.K2_GetActorLocation` _returnvalue)))
          (set `self.FinalFogAir` _data))
        (:`Is Not Valid`
          (`/Engine/EditorBlueprintResources/StandardMacros.IsValid` _previewfogactor
            (:`Is Valid`
              (set `self.FinalFogAir` (`/Game/Assets/InfinityWeather/Environment/Fog/BP_InfinityFog.Atmosphere` _previewfogactor)))
            (:`Is Not Valid`
              (set `self.FinalFogAir` (`self.AtmosphereSettings`)))))))
    (:`then_2`
      (`/Engine/EditorBlueprintResources/StandardMacros.IsValid` (`self.ExponentialHeightFog`)
        (:`Is Valid`
          (`ExponentialHeightFogComponent.SetFogDensity` _component _finalfogair_fogdensity)
          (`ExponentialHeightFogComponent.SetFogHeightFalloff` _component _finalfogair_fogheightfalloff)
          (`ExponentialHeightFogComponent.SetFogInscatteringColor` _component _finalfogair_fogcolor))))))

(fn `UpdateWindAffectedActors`
  (params (BlendDuration :type "Float (double-precision)"))
  (locals (ParticleSystem :type "ParticleSystemComponent Object Reference"))
  (`|ExecutionSequence`
    (:`then_0`
      (for _array_element (`self.WindAffectedEmitters`)
        (`/Engine/EditorBlueprintResources/StandardMacros.IsValid` _array_element
          (:`Is Valid`
            (set `local.ParticleSystem` (`Emitter.ParticleSystemComponent` _array_element))
            (`FXSystemComponent.SetVectorParameter` (`local.ParticleSystem`) "WindDirection" (`self.WindForceTo`))
            (`FXSystemComponent.SetFloatParameter` (`local.ParticleSystem`) "WindIntensity" (`KismetMathLibrary.VSize` (`self.WindForceTo`)))
            (if (`ActorComponent.ComponentHasTag` (`local.ParticleSystem`) "Directional")
              (`ActorComponent.SetActive` (`local.ParticleSystem`) (> (`KismetMathLibrary.Dot_VectorVector` (`self.WindForceTo`) (`KismetMathLibrary.Conv_RotatorToVector` (`SceneComponent.K2_GetComponentRotation` (`local.ParticleSystem`)))) 0.0) false))))))
    (:`then_1`
      (for _array_element_2 (`self.PrecipitationActors`)
        (`/Engine/EditorBlueprintResources/StandardMacros.IsValid` _array_element_2
          (:`Is Valid`
            (`/Game/Assets/InfinityWeather/Precipitation/Base/BP_InfinityPrecipitation.SetWindForce` _array_element_2 (`local.BlendDuration`) (`self.WindForceTo`))))))))

(fn `UpdateWindDirection`
  (params (DeltaTime :type "Float (double-precision)"))
  (locals (NewWindDirection :type "Vector2D Structure") (LWindDirection :type "Vector Structure") (LWindLength :type "Float (double-precision)"))
  (bind (_lwinddirection_x _lwinddirection_y _lwinddirection_z) (`KismetMathLibrary.BreakVector` (`local.LWindDirection`)))
  (bind (_lwinddirection_x_2 _lwinddirection_y_2) (`KismetMathLibrary.BreakVector` (`local.LWindDirection`)))
  (bind (_newwinddirection_x _newwinddirection_y) (`KismetMathLibrary.BreakVector2D` (`local.NewWindDirection`)))
  (bind (_returnvalue_x _returnvalue_y) (`KismetMathLibrary.BreakVector2D` (* (`local.NewWindDirection`) (-1.0 1.0))))
  (if (== DeltaTime -1.0)
    (set `local.LWindDirection` (`KismetMathLibrary.Conv_RotatorToVector` (`KismetMathLibrary.Conv_VectorToRotator` (`self.WindForce`))))
    (set `local.LWindLength` (`KismetMathLibrary.FMax` (`KismetMathLibrary.VSize` (`self.WindForce`)) 0.01))
    ;[1 1 1] Update parameters
    (`KismetMaterialLibrary.SetVectorParameterValue` "/Game/Assets/InfinityWeather/MPC_InfinityWeather.MPC_InfinityWeather" "WindForce" (make `LinearColor` _lwinddirection_x _lwinddirection_y _lwinddirection_z (`local.LWindLength`)) :!label _label)
    (set `local.NewWindDirection` (`KismetMathLibrary.MakeVector2D` _lwinddirection_x_2 _lwinddirection_y_2))
    (`AudioComponent.SetFloatParameter` (`self.WindAmbeint`) "Fade" (`local.LWindLength`))
    (if (== (`local.NewWindDirection`) (0.0 0.0))
      (set `local.NewWindDirection` (`self.SmallestWindDirection`))
      (else
        (set `self.SmallestWindDirection` (`local.NewWindDirection`))))
    (set `local.NewWindDirection` (`KismetMathLibrary.Normal2D` (`local.NewWindDirection`)))
    (`KismetMaterialLibrary.SetVectorParameterValue` "/Game/Assets/InfinityWeather/MPC_InfinityWeather.MPC_InfinityWeather" "WindBaseX" (make `LinearColor` _newwinddirection_x _newwinddirection_y 0.0 1.0))
    (`KismetMaterialLibrary.SetVectorParameterValue` "/Game/Assets/InfinityWeather/MPC_InfinityWeather.MPC_InfinityWeather" "WindBaseY" (make `LinearColor` _returnvalue_y _returnvalue_x 0.0 1.0))
    (elif (< (`self.WindBlendTime`) 1.0)
      (set `self.WindBlendTime` (`KismetMathLibrary.FMin` (+ (`self.WindBlendTime`) (* (`local.DeltaTime`) (`self.WindBlendSpeed`))) 1.0))
      (set `local.LWindDirection` (`KismetMathLibrary.Conv_RotatorToVector` (`KismetMathLibrary.RLerp` (`KismetMathLibrary.Conv_VectorToRotator` (`self.WindForceFrom`)) (`KismetMathLibrary.Conv_VectorToRotator` (`self.WindForceTo`)) (`self.WindBlendTime`))))
      (set `local.LWindLength` (`KismetMathLibrary.FMax` (`KismetMathLibrary.Lerp` (`KismetMathLibrary.Lerp` (`KismetMathLibrary.VSize` (`self.WindForceFrom`)) (`KismetMathLibrary.VSize` (`self.WindForceTo`)) (`self.WindBlendTime`)) (`KismetMathLibrary.VSize` (`KismetMathLibrary.VLerp` (`self.WindForceFrom`) (`self.WindForceTo`) (`self.WindBlendTime`))) 0.333) 0.01))
      (set `self.WindForce` (* (`local.LWindDirection`) (`local.LWindLength`)))
      (set `self.WindDamage` (`KismetMathLibrary.Lerp` (`self.WindDamageFrom`) (`self.WindDamageTo`) (`self.WindBlendTime`)))
      (goto _label))))

(fn `UpdateWindOffset`
  (params (DeltaTime :type "Float (double-precision)"))
  (bind (_windoffset_x _windoffset_y _windoffset_z) (`KismetMathLibrary.BreakVector` (`self.WindOffset`)))
  ;[1 1 1] Future effects can use this but need to be updated every flrame...
  (set `self.WindDistance` (+ (`self.WindDistance`) (* DeltaTime (`KismetMathLibrary.VSize` (`self.WindForce`)))))
  (set `self.WindOffset` (+ (`self.WindOffset`) (* (`self.WindForce`) DeltaTime)))
  (`KismetMaterialLibrary.SetVectorParameterValue` "/Game/Assets/InfinityWeather/MPC_InfinityWeather.MPC_InfinityWeather" "WindOffsetUV" (make `LinearColor` _windoffset_x _windoffset_y _windoffset_z (`self.WindDistance`))))

(fn `UserConstructionScript`
  (bind _windforce (`self.WindForce`))
  (set `self.WindOffset` (0.0 0.0 0.0))
  (`SceneComponent.K2_SetWorldRotation` (`self.WindDirection`) (`KismetMathLibrary.Conv_VectorToRotator` _windforce) false false)
  (`SceneComponent.SetWorldScale3D` (`self.WindDirection`) (`KismetMathLibrary.MakeVector` (`KismetMathLibrary.VSize` _windforce) 1.0 1.0))
  (`KismetArrayLibrary.Array_Clear` (`self.PrecipitationComponents`))
  (`KismetArrayLibrary.Array_Clear` (`self.PrecipitationActors`))
  (`self.SetDefault`)
  (bind _outactors (`GameplayStatics.GetAllActorsOfClass` "/Game/Assets/InfinityWeather/Precipitation/Base/BP_InfinityPrecipitation.BP_InfinityPrecipitation_C"))
  (for _array_element _outactors
    (`/Game/Assets/InfinityWeather/Precipitation/Base/BP_InfinityPrecipitation.SetWindForce` _array_element 0.0 (`self.WindForce`))))