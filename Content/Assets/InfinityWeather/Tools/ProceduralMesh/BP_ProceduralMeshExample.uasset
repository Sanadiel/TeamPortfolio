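; Example Blueprint from the InfinityWeather procedural mesh tools that builds a debug-textured plane when constructed.
; The Construction Script calls CreateMesh, which generates a plane definition, writes it to the ProceduralMesh component, logs its stats and applies a grid material.
; An unconnected alternative chain demonstrates combining meshes by transforming one quad and appending it to another.
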(fn `CreateMesh`
  ;[1 1 1] Create simple plane
  (bind _mesh (`/Game/Assets/InfinityWeather/Tools/ProceduralMesh/BPL_ProceduralMesh.BuildPlane` (100.0 100.0) 2 8))
  (`/Game/Assets/InfinityWeather/Tools/ProceduralMesh/BPL_ProceduralMesh.CreateMeshSection` (`self.ProceduralMesh`) _mesh)
  (`/Game/Assets/InfinityWeather/Tools/ProceduralMesh/BPL_ProceduralMesh.LogStats` _mesh)
  (`PrimitiveComponent.SetMaterial` (`self.ProceduralMesh`) 0 "/Game/Assets/InfinityWeather/Tools/ProceduralMesh/M_DebugGrid.M_DebugGrid"))

(fn `UserConstructionScript`
  (`self.CreateMesh`))