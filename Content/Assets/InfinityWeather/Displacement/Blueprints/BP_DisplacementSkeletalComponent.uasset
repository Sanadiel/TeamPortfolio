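; BP_DisplacementSkeletalComponent supplies Infinity Weather displacement shapes that follow the bones of a skeletal mesh.
; AddDisplacementShapeData optionally appends fast spheres and body capsules, each defined by bone pairs and radii from class defaults.
; Body capsules span their two bones.
; Fast spheres track bone midpoints between updates, stretching into capsules along the movement when its length is within range, otherwise remaining point shapes.
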(event `self.ReceiveBeginPlay`
  (bind _bodycapsules (`self.BodyCapsules`))
  (if (`KismetSystemLibrary.IsValidClass` _bodycapsules)
    (`KismetArrayLibrary.Array_Resize` (`self.PreviousLocations`) (`KismetArrayLibrary.Array_Length` (defaults `Object` _bodycapsules)))
    (set `self.InitializeFastSpheres` true)))

(fn `AddBodyCapsules`
  (params (Shapes :type "Array of /Game/Assets/InfinityWeather/Displacement/Blueprints/BS_DisplacementShape Structure") (Mesh :type "SceneComponent Object Reference"))
  (locals (Result :type "Array of /Game/Assets/InfinityWeather/Displacement/Blueprints/BS_DisplacementShape Structure") (Center :type "Vector Structure" :default (0.0 0.0 0.0)) (A :type "Vector Structure" :default (0.0 0.0 0.0)) (B :type "Vector Structure" :default (0.0 0.0 0.0)) (Shape :type "/Game/Assets/InfinityWeather/Displacement/Blueprints/BS_DisplacementBone Structure"))
  (bind _mesh (`local.Mesh`))
  (bind _bodycapsules (`self.BodyCapsules`))
  (bind (_shape_bonestart _shape_boneend) (break `/Game/Assets/InfinityWeather/Displacement/Blueprints/BS_DisplacementBone` (`local.Shape`)))
  (bind (_shape_bonestart_2 _shape_boneend_2 _shape_radius) (break `/Game/Assets/InfinityWeather/Displacement/Blueprints/BS_DisplacementBone` (`local.Shape`)))
  (bind _returnvalue (- (`local.A`) (`local.B`)))
  ;[1 1 1] Body capsules
  (if (and (`self.UseBodyCapsules`) (`KismetSystemLibrary.IsValidClass` _bodycapsules))
    (for _array_element (defaults `Object` _bodycapsules)
      (set `local.Shape` _array_element)
      (set `local.A` (`SceneComponent.GetSocketLocation` _mesh _shape_bonestart))
      (set `local.B` (`SceneComponent.GetSocketLocation` _mesh _shape_boneend))
      (`KismetArrayLibrary.Array_Add` (`local.Shapes`) (make `/Game/Assets/InfinityWeather/Displacement/Blueprints/BS_DisplacementShape` null "NewEnumerator5" (`KismetMathLibrary.MakeTransform` (`KismetMathLibrary.VLerp` (`local.A`) (`local.B`) 0.5) (`KismetMathLibrary.MakeRotFromZ` _returnvalue) (`KismetMathLibrary.MakeVector` _shape_radius _shape_radius (* (`KismetMathLibrary.VSize` _returnvalue) 0.5))))))
    (else
      (return))))

(fn `AddDisplacementShapeData`
  (params (Shapes :type "Array of /Game/Assets/InfinityWeather/Displacement/Blueprints/BS_DisplacementShape Structure (by ref)") (SceneComponent :type "SceneComponent Object Reference"))
  (locals (Result :type "Array of /Game/Assets/InfinityWeather/Displacement/Blueprints/BS_DisplacementShape Structure") (Center :type "Vector Structure" :default (0.0 0.0 0.0)) (A :type "Vector Structure" :default (0.0 0.0 0.0)) (B :type "Vector Structure" :default (0.0 0.0 0.0)) (Shape :type "/Game/Assets/InfinityWeather/Displacement/Blueprints/BS_DisplacementBone Structure") (Next :type "Vector Structure") (Prev :type "Vector Structure") (Length :type "Float (double-precision)"))
  (`|ExecutionSequence`
    (:`then_0`
      (if (`self.UseFastSpheres`)
        (`self.AddFastSpheres` (`local.Shapes`) (`local.SceneComponent`))))
    (:`then_1`
      (if (`self.UseBodyCapsules`)
        (`self.AddBodyCapsules` (`local.Shapes`) (`local.SceneComponent`))))))

(fn `AddFastSpheres`
  (params (Shapes :type "Array of /Game/Assets/InfinityWeather/Displacement/Blueprints/BS_DisplacementShape Structure (by ref)") (Mesh :type "SceneComponent Object Reference"))
  (locals (Next :type "Vector Structure") (Prev :type "Vector Structure") (Direction :type "Vector Structure") (Shape :type "/Game/Assets/InfinityWeather/Displacement/Blueprints/BS_DisplacementBone Structure") (Length :type "Float (double-precision)" :default 0.0))
  (bind (_shape_bonestart _shape_boneend _shape_radius) (break `/Game/Assets/InfinityWeather/Displacement/Blueprints/BS_DisplacementBone` (`local.Shape`)))
  (bind (_minmaxfastspherelength_x _minmaxfastspherelength_y) (`KismetMathLibrary.BreakVector2D` (`self.MinMaxFastSphereLength`)))
  (bind (_shape_bonestart_2 _shape_boneend_2 _shape_radius_2) (break `/Game/Assets/InfinityWeather/Displacement/Blueprints/BS_DisplacementBone` (`local.Shape`)))
  (bind (_shape_bonestart_3 _shape_boneend_3) (break `/Game/Assets/InfinityWeather/Displacement/Blueprints/BS_DisplacementBone` (`local.Shape`)))
  (bind _mesh (`local.Mesh`))
  (bind _mesh_2 (`local.Mesh`))
  (bind (_shape_bonestart_4 _shape_boneend_4) (break `/Game/Assets/InfinityWeather/Displacement/Blueprints/BS_DisplacementBone` (`local.Shape`)))
  (if (`self.InitializeFastSpheres`)
    ;[1 1 1] Init previous state
    (for (_array_element _array_index) (defaults `Object` (`self.FastSpheres`))
      (set `local.Shape` _array_element)
      (`KismetArrayLibrary.Array_Set` (`self.PreviousLocations`) _array_index (`KismetMathLibrary.VLerp` (`SceneComponent.GetSocketLocation` _mesh_2 _shape_bonestart_4) (`SceneComponent.GetSocketLocation` _mesh_2 _shape_boneend_4) 0.5) true))
    (set `self.InitializeFastSpheres` false))
  (for (_array_element_2 _array_index_2) (defaults `Object` (`self.FastSpheres`))
    (set `local.Shape` _array_element_2)
    (set `local.Next` (`KismetMathLibrary.VLerp` (`SceneComponent.GetSocketLocation` _mesh _shape_bonestart_3) (`SceneComponent.GetSocketLocation` _mesh _shape_boneend_3) 0.5))
    (set `local.Prev` (`|GetArrayItem` (`self.PreviousLocations`) _array_index_2))
    (set `local.Direction` (- (`local.Next`) (`local.Prev`)))
    (set `local.Length` (`KismetMathLibrary.VSize` (`local.Direction`)))
    (if (`KismetMathLibrary.InRange_FloatFloat` (`local.Length`) _minmaxfastspherelength_x _minmaxfastspherelength_y)
      (`KismetArrayLibrary.Array_Add` (`local.Shapes`) (make `/Game/Assets/InfinityWeather/Displacement/Blueprints/BS_DisplacementShape` null "NewEnumerator5" (`KismetMathLibrary.MakeTransform` (`KismetMathLibrary.VLerp` (`local.Next`) (`local.Prev`) 0.5) (`KismetMathLibrary.MakeRotFromZ` (`local.Direction`)) (`KismetMathLibrary.MakeVector` _shape_radius_2 _shape_radius_2 (* (`local.Length`) 0.5)))))
      (else
        (`KismetArrayLibrary.Array_Add` (`local.Shapes`) (make `/Game/Assets/InfinityWeather/Displacement/Blueprints/BS_DisplacementShape` null "NewEnumerator0" (`KismetMathLibrary.MakeTransform` (`local.Next`) (struct) (`KismetMathLibrary.Conv_DoubleToVector` _shape_radius))))))
    (`KismetArrayLibrary.Array_Set` (`self.PreviousLocations`) _array_index_2 (`local.Next`))))