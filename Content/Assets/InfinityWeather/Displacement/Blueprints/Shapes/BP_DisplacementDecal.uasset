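; BP_DisplacementDecal is a texture-based displacement shape actor in the InfinityWeather displacement assets, exposing its texture through GetDisplacementTexture.
; The construction script applies that texture to a dynamic M_DecalPreview material on the static mesh and toggles the mesh's visibility with EditorPreview.
; On BeginPlay it hides the Box component and, if LifeTime is positive, destroys itself after that delay.
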(event `self.ReceiveBeginPlay`
  (bind _box (`self.Box`))
  (`parent.ReceiveBeginPlay`)
  (`/Engine/EditorBlueprintResources/StandardMacros.IsValid` _box
    (:`Is Valid`
      (`SceneComponent.SetVisibility` _box false false)
      (if (> (`self.LifeTime`) 0.0)
        (`KismetSystemLibrary.Delay` (`self.LifeTime`))
        (`self.K2_DestroyActor`)))))

(fn `GetDisplacementTexture`
  (returns (Texture :type "Texture2D Object Reference"))
  (return (`self.Texture`)))

(fn `UserConstructionScript`
  (`parent.UserConstructionScript`)
  (bind _returnvalue (`PrimitiveComponent.CreateDynamicMaterialInstance` (`self.StaticMeshComponent`) 0 "/Game/Assets/InfinityWeather/Displacement/Capture/M_DecalPreview.M_DecalPreview" "None"))
  (`MaterialInstanceDynamic.SetTextureParameterValue` _returnvalue "Texture" (`self.Texture`))
  (`SceneComponent.SetVisibility` (`self.StaticMeshComponent`) (`self.EditorPreview`) false))